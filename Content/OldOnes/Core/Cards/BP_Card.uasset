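; BP_Card is the runtime representation of a card, built from a card data struct and able to pack itself back into one.
; It adds an ability manager to its owner, delegating targeting and execution to it, and binds to its targets-ready event.
; CardReadyForPlay submits the card to the player pawn with mana payment.
; Mana and location changes fire dispatchers, while ModifyCard copies another card's data only when IDs match.
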(fn `CardReadyForPlay`
  (params (FiringAbilityManager :type "/Game/OldOnes/Core/Abilities/BP_AbilityManager Object Reference"))
  (`/Game/OldOnes/Core/Player/BP_PlayerPawn.CardReadyForPlay` (`/Game/OldOnes/Core/Tools/BPFL_GeneralFunctions.GetCardPlayerPawn`) self true))

(fn `ChangeLocation`
  (params (NewLocation :type "/Game/OldOnes/Core/Cards/ECardLocation Enum" :default "NewEnumerator0"))
  (set `self.CardLocation` NewLocation)
  (`self.SendCardToLocation` NewLocation))

(fn `ChangeManaValue`
  (params (NewValue :type Integer))
  (if (!= NewValue (`self.ManaCost`))
    (bind _output_get (set `self.ManaCost` NewValue))
    (`self.ManaValueChanged` _output_get)))

(fn `Get Abilities`
  (returns (Abilities :type "/Game/OldOnes/Core/Abilities/BP_AbilityManager Object Reference"))
  (return (`self.Abilities`)))

(fn `GetCardType`
  (returns (CardType :type "/Game/OldOnes/Core/Cards/ECardTypes Enum"))
  (return (`self.CardType`)))

(fn `GetManaValue`
  (returns (ManaValue :type Integer))
  (return (`self.ManaCost`)))

(fn `GetName`
  (returns (Name :type String))
  (return (`self.Name`)))

(fn `GetTargets`
  (`/Game/OldOnes/Core/Abilities/BP_AbilityManager.GetTargets` (`self.Abilities`)))

(fn `Initialize Card From Struct`
  (params (CardStruct :type "/Game/OldOnes/Core/Cards/SCardData Structure"))
  (returns (InitializedCard :type "/Game/OldOnes/Core/Cards/BP_Card Object Reference"))
  (locals (AbilitiesArray :type "Array of /Game/OldOnes/Core/Abilities/BP_AbilityInterface Object Reference"))
  (bind (_name _manacost _cardtype _cardclass _abilities _illustration) (break `/Game/OldOnes/Core/Cards/SCardData` CardStruct))
  (bind _returnvalue (`|AddComponentByClass` (`self.GetOwner`) "/Game/OldOnes/Core/Abilities/BP_AbilityManager.BP_AbilityManager_C"))
  (bind _output_get (set `self.Abilities` _returnvalue))
  (add `/Game/OldOnes/Core/Abilities/BP_AbilityManager.TargetsReadyForExecution` _output_get (`|CreateDelegate` :!event `CardReadyForPlay`))
  (set `self.Name` _name)
  (set `self.ManaCost` _manacost)
  (set `self.CardType` _cardtype)
  (set `self.CardClass` _cardclass)
  (`/Game/OldOnes/Core/Abilities/BP_AbilityManager.AddAbilities` (`self.Abilities`) _abilities)
  (set `self.Illustration` _illustration)
  (return self))

(fn `ModifyCard`
  (params (CardToModifyTo :type "/Game/OldOnes/Core/Cards/BP_Card Object Reference"))
  (bind (_name _manacost _cardtype _cardclass _abilities _illustration _cardid) (break `/Game/OldOnes/Core/Cards/SCardData` (`self.PackCardToStruct` CardToModifyTo)))
  (if (== (`self.CardUniqueID`) _cardid)
    (set `self.Name` _name)
    (set `self.ManaCost` _manacost)
    (set `self.CardType` _cardtype)
    (set `self.CardClass` _cardclass)
    (set `self.Illustration` _illustration)
    (`/Game/OldOnes/Core/Abilities/BP_AbilityManager.ModifyAbilityManager` (`self.Abilities`) _abilities)
    (else
      (`KismetSystemLibrary.PrintString` "BP_Card::ModifyCard Trying to modify a card with another card" true true (struct :`R` 1.0 :`A` 1.0) 30.0))))

(fn `PackCardToStruct`
  (returns (CardStruct :type "/Game/OldOnes/Core/Cards/SCardData Structure"))
  (return (make `/Game/OldOnes/Core/Cards/SCardData` (`self.Name`) (`self.ManaCost`) (`self.CardType`) (`self.CardClass`) (`/Game/OldOnes/Core/Abilities/BP_AbilityManager.PackAbilitiesToStruct` (`self.Abilities`)) (`self.Illustration`) (`self.CardUniqueID`))))

(fn `PlayCard`
  (`/Game/OldOnes/Core/Abilities/BP_AbilityManager.ExecuteAbilities` (`self.Abilities`)))