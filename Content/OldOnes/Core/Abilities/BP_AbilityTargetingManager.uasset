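; Resolves card ability targets (player, cards, enemies, investigables) from gameplay tags for the card game.
; QueryForTargets dispatches by targeting style to specific, random, all, self, by-name or no-target handlers, storing results in an indexed TargetsQueue.
; Specific targeting prompts the player and collects clicks through bound events, while other styles resolve immediately.
; Completion fires TargetingDone for BP_AbilityBase; queued sequential targeting and all-investigables targeting are unimplemented.
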(event `self.ReceiveBeginPlay`
  (add `self.TargetingDoneEvent` (delegate `GoToNextTargetManagementInQueue`))
  (`KismetArrayLibrary.Array_Resize` (`self.TargetsQueue`) 10))

(event `GoToNextTargetManagementInQueue` :!signature `self.TargetingDoneEvent`
  (params (Targets :type "/Game/OldOnes/Core/Abilities/STargetsArray Structure") (IndexOfTargetsInQueue :type Integer))
  (`KismetSystemLibrary.PrintString` "AbilityTargetingManager::EventGraph: There is no waiting queue all targets are done in a row. This will be an issue if multiple specifictargets in one card"))

(fn `AllCardsHandler`
  (params (TargetsTags :type "Array of /Game/OldOnes/Core/Abilities/SAbilityAttribute Structure") (QueueIndex :type Integer))
  (bind _foundcards (`/Game/OldOnes/Core/Tools/BPFL_Cards.FindCardsFromAbilityStruct` TargetsTags))
  (bind _mergedresults (`/Game/OldOnes/Core/Tools/BPFL_Cards.GetMergedArrayFromResults` _foundcards))
  (`self.SetTargetQueueTargetsAtIndex` QueueIndex _mergedresults))

(fn `AllEnemyHandler`
  (params (TargetsTags :type "Array of /Game/OldOnes/Core/Abilities/SAbilityAttribute Structure") (QueueIndex :type Integer))
  (bind _enemies (`/Game/OldOnes/Core/Tools/BPFL_Targeting.GetAllEnemies`))
  (`self.SetTargetQueueTargetsAtIndex` QueueIndex _enemies))

(fn `AllInvestigableHandler`
  (params (TargetsTags :type "Array of /Game/OldOnes/Core/Abilities/SAbilityAttribute Structure") (QueueIndex :type Integer))
  (`KismetSystemLibrary.PrintString` "BP_AbilityTargetingManager::SpecificCardHandler NotImplemented Yet"))

(fn `AllTargetsHandler`
  (params (TargetsTags :type "Array of /Game/OldOnes/Core/Abilities/SAbilityAttribute Structure") (QueueIndex :type Integer))
  (bind _targetstags (`local.TargetsTags`))
  (bind _queueindex (`local.QueueIndex`))
  (if (`/Game/OldOnes/Core/Abilities/BPFL_AbilityAttributeParser.HasTag` TargetsTags (struct :`TagName` "TargetingStyle.Card"))
    (`self.AllCardsHandler` _targetstags _queueindex)
    (elif (`/Game/OldOnes/Core/Abilities/BPFL_AbilityAttributeParser.HasTag` TargetsTags (struct :`TagName` "TargetingStyle.Enemy"))
      (`self.AllEnemyHandler` _targetstags _queueindex)
      (elif (`/Game/OldOnes/Core/Abilities/BPFL_AbilityAttributeParser.HasTag` TargetsTags (struct :`TagName` "TargetingStyle.Investigable"))
        (`self.AllInvestigableHandler` _targetstags _queueindex)
        (else
          (`KismetSystemLibrary.PrintString` "BP_AbilityTargetingManager::AllTargetsHandler: Target Type not handled"))))))

(fn `CardsTargetsText`
  (params (NumberOfTargets :type Integer) (AreTargetsDifferent :type Boolean))
  (returns (Text :type Text))
  (locals (Repeatable :type Text) (`Card(s)` :type Text))
  (if (> NumberOfTargets 1)
    (set `local.Card(s)` "s"))
  (if (not (`local.AreTargetsDifferent`))
    (set `local.Repeatable` " You can choose the same more than once."))
  (return (`|FormatText` "Choose {X} card{Ys}.{Repeatable}" (`local.NumberOfTargets`) (`local.Card(s)`) (`local.Repeatable`))))

(fn `EnemyTargetsText`
  (params (NumberOfTargets :type Integer) (AreTargetsDifferent :type Boolean))
  (returns (Text :type Text))
  (locals (Different :type Text) (Ennemyies :type Text))
  (if (> NumberOfTargets 1)
    (set `local.Ennemyies` "ies")
    (if (`local.AreTargetsDifferent`)
      (set `local.Different` "different "))
    (else
      (set `local.Ennemyies` "y")))
  (return (`|FormatText` "Target {X} {Different}enem{Ys}." (`local.NumberOfTargets`) (`local.Different`) (`local.Ennemyies`))))

(fn `InvestigableTargetsText`
  (params (NumberOfTargets :type Integer) (AreTargetsDifferent :type Boolean))
  (returns (Text :type Text))
  (locals (Different :type Text) (`Investigable(S)` :type Text))
  (if (> NumberOfTargets 1)
    (set `local.Investigable(S)` "s")
    (if (`local.AreTargetsDifferent`)
      (set `local.Different` "different ")))
  (return (`|FormatText` "Target {X} {Different}investigable{s}." (`local.NumberOfTargets`) (`local.Different`) (`local.Investigable(S)`))))

(fn `NamedCardHandler`
  (params (TargetsTags :type "Array of /Game/OldOnes/Core/Abilities/SAbilityAttribute Structure") (CardNameAttribute :type "/Game/OldOnes/Core/Abilities/SAbilityAttribute Structure") (QueueIndex :type Integer))
  (locals (NumberCardsFound :type Integer) (NbCardsToFind :type Integer) (CardsTargeted :type "Array of /Game/OldOnes/Core/Cards/BP_Card Object Reference"))
  (bind (_attributevalue _attributetags _specialabilitycardname) (break `/Game/OldOnes/Core/Abilities/SAbilityAttribute` CardNameAttribute))
  (if (> _attributevalue 0)
    (set `local.NbCardsToFind` _attributevalue)
    (bind _foundcards (`/Game/OldOnes/Core/Tools/BPFL_Cards.FindCardsFromAbilityStruct` TargetsTags))
    (bind _mergedresults (`/Game/OldOnes/Core/Tools/BPFL_Cards.GetMergedArrayFromResults` _foundcards))
    (for _array_element _mergedresults
      (if (`KismetStringLibrary.EqualEqual_StrStr` (`/Game/OldOnes/Core/Cards/BP_Card.GetName` _array_element) _specialabilitycardname)
        (`KismetArrayLibrary.Array_Add` (`local.CardsTargeted`) _array_element)
        (bind _result (`/Engine/EditorBlueprintResources/StandardMacros.IncrementInt` (`local.NumberCardsFound`))
          (:`  `
            (if (== _result (`local.NbCardsToFind`))
              (break))))))
    (`self.SetTargetQueueTargetsAtIndex` (`local.QueueIndex`) (`local.CardsTargeted`))
    (else
      (`KismetSystemLibrary.PrintString` "BP_AbilityTargetingManager::NamedCardHandler: You probably forgot to put a number attribute in your named card targeting style" true true (struct :`A` 1.0) 20.0))))

(fn `NoTargetHandler`
  (params (IndexInQueue :type Integer))
  (`self.SetTargetQueueTargetsAtIndex` IndexInQueue (`|MakeArray` null :!type "Object Object Reference")))

(fn `PlayerTargetHandler`
  (params (QueueIndex :type Integer))
  (`self.SetTargetQueueTargetsAtIndex` QueueIndex (`|MakeArray` (`/Game/OldOnes/Core/Tools/BPFL_GeneralFunctions.GetCardPlayerPawn`) :!type "Object Object Reference")))

(fn `QueryForTargets`
  (params (TargetsTags :type "Array of /Game/OldOnes/Core/Abilities/SAbilityAttribute Structure") (QueueIndex :type Integer))
  (bind (_hastag _tagattributevalue _foundattribute) (`/Game/OldOnes/Core/Abilities/BPFL_AbilityAttributeParser.HasTag` (`local.TargetsTags`) (struct :`TagName` "TargetingStyle.Card.ByName")))
  (if (== QueueIndex 0)
    (`KismetArrayLibrary.Array_Clear` (`self.TargetsQueue`)))
  (if (`/Game/OldOnes/Core/Abilities/BPFL_AbilityAttributeParser.HasTag` (`local.TargetsTags`) (struct :`TagName` "TargetingStyle.Player"))
    (`self.PlayerTargetHandler` (`local.QueueIndex`))
    (elif (`/Game/OldOnes/Core/Abilities/BPFL_AbilityAttributeParser.HasAny` (`local.TargetsTags`) (`BlueprintGameplayTagLibrary.MakeGameplayTagContainerFromArray` (`|MakeArray` (struct :`TagName` "TargetingStyle.Card.Specific") (struct :`TagName` "TargetingStyle.Enemy.Specific") (struct :`TagName` "TargetingStyle.Investigable.Specific") :!type "GameplayTag Structure")))
      (`self.SpecificTargetsHandler` (`local.TargetsTags`) (`local.QueueIndex`))
      (elif (`/Game/OldOnes/Core/Abilities/BPFL_AbilityAttributeParser.HasAny` (`local.TargetsTags`) (`BlueprintGameplayTagLibrary.MakeGameplayTagContainerFromArray` (`|MakeArray` (struct :`TagName` "TargetingStyle.Card.Random") (struct :`TagName` "TargetingStyle.Enemy.Random") (struct :`TagName` "TargetingStyle.Investigable.Random") :!type "GameplayTag Structure")))
        (`self.RandomTargetsHandler` (`local.TargetsTags`) (`local.QueueIndex`))
        (elif (`/Game/OldOnes/Core/Abilities/BPFL_AbilityAttributeParser.HasAny` (`local.TargetsTags`) (`BlueprintGameplayTagLibrary.MakeGameplayTagContainerFromArray` (`|MakeArray` (struct :`TagName` "TargetingStyle.Card.All") (struct :`TagName` "TargetingStyle.Enemy.All") (struct :`TagName` "TargetingStyle.Investigable.All") :!type "GameplayTag Structure")))
          (`self.AllTargetsHandler` (`local.TargetsTags`) (`local.QueueIndex`))
          (elif (`/Game/OldOnes/Core/Abilities/BPFL_AbilityAttributeParser.HasAny` (`local.TargetsTags`) (`BlueprintGameplayTagLibrary.MakeGameplayTagContainerFromArray` (`|MakeArray` (struct :`TagName` "TargetingStyle.Card.Self") (struct :`TagName` "TargetingStyle.Enemy.Self") :!type "GameplayTag Structure")))
            (`self.SelfTargetingHandler` (`local.TargetsTags`) (`local.QueueIndex`))
            (elif _hastag
              (`self.NamedCardHandler` (`local.TargetsTags`) _foundattribute (`local.QueueIndex`))
              (elif (not (`/Game/OldOnes/Core/Abilities/BPFL_AbilityAttributeParser.HasTag` (`local.TargetsTags`) (struct :`TagName` "TargetingStyle")))
                (`self.NoTargetHandler` (`local.QueueIndex`))
                (else
                  (`KismetSystemLibrary.PrintString` "BP_abilityTargetingManager::QueryTargets: No Targetting style found. Strange" true true (struct :`G` 0.66 :`B` 1.0 :`A` 1.0) 20.0))))))))))

(fn `RandomCardHandler`
  (params (TargetsTags :type "Array of /Game/OldOnes/Core/Abilities/SAbilityAttribute Structure") (NumberOfTargets :type Integer) (QueueIndex :type Integer))
  (bind _foundcards (`/Game/OldOnes/Core/Tools/BPFL_Cards.FindCardsFromAbilityStruct` TargetsTags))
  (bind _mergedresults (`/Game/OldOnes/Core/Tools/BPFL_Cards.GetMergedArrayFromResults` _foundcards))
  (bind _randomobjects (`/Game/OldOnes/Core/Tools/BPFL_Targeting.GetRandomObjectsFromArray` _mergedresults NumberOfTargets (not (`/Game/OldOnes/Core/Abilities/BPFL_AbilityAttributeParser.HasTag` TargetsTags (struct :`TagName` "TargetRestriction.RepeatableTargets")))))
  (`self.SetTargetQueueTargetsAtIndex` (`local.QueueIndex`) _randomobjects))

(fn `RandomEnemyHandler`
  (params (TargetsTags :type "Array of /Game/OldOnes/Core/Abilities/SAbilityAttribute Structure") (NumberOfTargets :type Integer) (QueueIndex :type Integer))
  (bind _randomenemies (`/Game/OldOnes/Core/Tools/BPFL_Targeting.GetRandomEnemies` NumberOfTargets (not (`/Game/OldOnes/Core/Abilities/BPFL_AbilityAttributeParser.HasTag` TargetsTags (struct :`TagName` "TargetRestriction.RepeatableTargets") true))))
  (`self.SetTargetQueueTargetsAtIndex` QueueIndex _randomenemies))

(fn `RandomInvestigableHandler`
  (params (TargetsTags :type "Array of /Game/OldOnes/Core/Abilities/SAbilityAttribute Structure") (NumberOfTargets :type Integer) (QueueIndex :type Integer))
  (bind _randominvestigables (`/Game/OldOnes/Core/Tools/BPFL_Targeting.GetRandomInvestigables` NumberOfTargets (not (`/Game/OldOnes/Core/Abilities/BPFL_AbilityAttributeParser.HasTag` TargetsTags (struct :`TagName` "TargetRestriction.RepeatableTargets") true))))
  (`self.SetTargetQueueTargetsAtIndex` QueueIndex _randominvestigables))

(fn `RandomTargetsHandler`
  (params (TargetsTags :type "Array of /Game/OldOnes/Core/Abilities/SAbilityAttribute Structure") (QueueIndex :type Integer))
  (bind (_hastag _tagattributevalue) (`/Game/OldOnes/Core/Abilities/BPFL_AbilityAttributeParser.HasTag` TargetsTags (struct :`TagName` "TargetingStyle.Enemy")))
  (bind (_hastag_2 _tagattributevalue_2) (`/Game/OldOnes/Core/Abilities/BPFL_AbilityAttributeParser.HasTag` TargetsTags (struct :`TagName` "TargetingStyle.Investigable")))
  (bind (_hastag_3 _tagattributevalue_3) (`/Game/OldOnes/Core/Abilities/BPFL_AbilityAttributeParser.HasTag` TargetsTags (struct :`TagName` "TargetingStyle.Card")))
  (bind _targetstags (`local.TargetsTags`))
  (bind _queueindex (`local.QueueIndex`))
  (if _hastag_3
    (`self.RandomCardHandler` _targetstags _tagattributevalue_3 _queueindex)
    (elif _hastag
      (`self.RandomEnemyHandler` _targetstags _tagattributevalue _queueindex)
      (elif _hastag_2
        (`self.RandomInvestigableHandler` _targetstags _tagattributevalue_2 _queueindex)
        (else
          (`KismetSystemLibrary.PrintString` "BP_AbilityTargetingManager::SpecifcTargetHandler: Type of object targetable not supported" true true (struct :`G` 0.66 :`B` 1.0 :`A` 1.0) 10.0))))))

(fn `Receive Enemy Clicked Event`
  (params (EnemyClicked :type "/Game/OldOnes/Core/Enemy/BP_Enemy Object Reference"))
  (locals (LocalTargetsArray :type "/Game/OldOnes/Core/Abilities/STargetsArray Structure"))
  (if (`self.AreTargetsUnique`)
    (if (not (`KismetArrayLibrary.Array_Contains` (`.Targets_3_335D2E364641915E317A669DF93277B1` (break `/Game/OldOnes/Core/Abilities/STargetsArray` (`|GetArrayItem` (`self.TargetsQueue`) (`self.TargetsQueueIndex`)))) EnemyClicked))
      (`KismetArrayLibrary.Array_Add` (`.Targets_3_335D2E364641915E317A669DF93277B1` (break `/Game/OldOnes/Core/Abilities/STargetsArray` (`|GetArrayItem` (`self.TargetsQueue`) (`self.TargetsQueueIndex`)))) (`local.EnemyClicked`) :!label _label)
      (bind _result (`/Engine/EditorBlueprintResources/StandardMacros.DecrementInt` (`self.NumberOfTargetsToGet`))
        (:`  `
          (if (== _result 0)
            (remove `/Game/OldOnes/Core/Player/BP_CardPlayerController.EnemyClickedEvent` (`/Game/OldOnes/Core/Tools/BPFL_GeneralFunctions.GetCardPlayerController`) (`|CreateDelegate` :!event `Receive Enemy Clicked Event`))
            (`self.TargetingDoneEvent` (`|GetArrayItem` (`self.TargetsQueue`) (`self.TargetsQueueIndex`)) (`self.TargetsQueueIndex`)) ; Event caught by BP_AbilityBase
            (`/Game/OldOnes/Core/Tools/BPFL_WidgetUtilities.Display Message to User` "") ; Hide text
            (else
              (bind _text (`self.EnemyTargetsText` (`self.NumberOfTargetsToGet`) (`self.AreTargetsUnique`))) ; More Targets to select
              (`/Game/OldOnes/Core/Tools/BPFL_WidgetUtilities.Display Message to User` _text)))))
      (else
        (`/Game/OldOnes/Core/Tools/BPFL_WidgetUtilities.Display Message to User` "Enemy Already selected, please get another Target")))
    (else
      (goto _label))))

(fn `ReceiveCardTargetedEvent`
  (params (CardTargeted :type "/Game/OldOnes/Core/PlayerUI/WBP_CardView Object Reference"))
  (if (`self.AreTargetsUnique`)
    (if (not (`KismetArrayLibrary.Array_Contains` (`.Targets_3_335D2E364641915E317A669DF93277B1` (break `/Game/OldOnes/Core/Abilities/STargetsArray` (`|GetArrayItem` (`self.TargetsQueue`) (`self.TargetsQueueIndex`)))) (`/Game/OldOnes/Core/PlayerUI/WBP_CardView.ViewedCard` CardTargeted)))
      (`KismetArrayLibrary.Array_Add` (`.Targets_3_335D2E364641915E317A669DF93277B1` (break `/Game/OldOnes/Core/Abilities/STargetsArray` (`|GetArrayItem` (`self.TargetsQueue`) (`self.TargetsQueueIndex`)))) (`/Game/OldOnes/Core/PlayerUI/WBP_CardView.ViewedCard` (`local.CardTargeted`)) :!label _label)
      (bind _result (`/Engine/EditorBlueprintResources/StandardMacros.DecrementInt` (`self.NumberOfTargetsToGet`))
        (:`  `
          (if (== _result 0)
            (for _array_element (`self.SelectableCards`)
              (`/Game/OldOnes/Core/PlayerUI/WBP_CardView.ToggleTargetable` _array_element false)
              (remove `/Game/OldOnes/Core/PlayerUI/WBP_CardView.CardTargetedEvent` _array_element (`|CreateDelegate` :!event `ReceiveCardTargetedEvent`))
              (`/Game/OldOnes/Core/PlayerUI/WBP_CardCollectionView.ResetCollectionView` (`/Game/OldOnes/Core/PlayerUI/WBP_GameUI.CardCollectionView` (`/Game/OldOnes/Core/Tools/BPFL_GeneralFunctions.GetPlayerUI`)))
              (`self.TargetingDoneEvent` (`|GetArrayItem` (`self.TargetsQueue`) (`self.TargetsQueueIndex`)) (`self.TargetsQueueIndex`)) ; Event caught by BP_AbilityBase
              (`/Game/OldOnes/Core/Tools/BPFL_WidgetUtilities.Display Message to User` "") ; Hide text
            )
            (else
              (bind _text (`self.CardsTargetsText` (`self.NumberOfTargetsToGet`) (`self.AreTargetsUnique`)))
              (`/Game/OldOnes/Core/Tools/BPFL_WidgetUtilities.Display Message to User` _text)))))
      (else
        (`/Game/OldOnes/Core/Tools/BPFL_WidgetUtilities.Display Message to User` "Card Already selected, please get another Target")))
    (else
      (goto _label))))

(fn `ReceiveInvestigableClickedEvent`
  (params (InvestigableClicked :type "/Game/OldOnes/Core/Investigable/BP_Investigable Object Reference"))
  (if (`self.AreTargetsUnique`)
    (if (== (`KismetArrayLibrary.Array_Find` (`.Targets_3_335D2E364641915E317A669DF93277B1` (break `/Game/OldOnes/Core/Abilities/STargetsArray` (`|GetArrayItem` (`self.TargetsQueue`) (`self.TargetsQueueIndex`)))) InvestigableClicked) -1)
      (`KismetArrayLibrary.Array_Add` (`.Targets_3_335D2E364641915E317A669DF93277B1` (break `/Game/OldOnes/Core/Abilities/STargetsArray` (`|GetArrayItem` (`self.TargetsQueue`) (`self.TargetsQueueIndex`)))) (`local.InvestigableClicked`) :!label _label)
      (bind _result (`/Engine/EditorBlueprintResources/StandardMacros.DecrementInt` (`self.NumberOfTargetsToGet`))
        (:`  `
          (if (== _result 0)
            (remove `/Game/OldOnes/Core/Player/BP_CardPlayerController.InvestigableClickedEvent` (`/Game/OldOnes/Core/Tools/BPFL_GeneralFunctions.GetCardPlayerController`) (`|CreateDelegate` :!event `ReceiveInvestigableClickedEvent`))
            (`self.TargetingDoneEvent` (`|GetArrayItem` (`self.TargetsQueue`) (`self.TargetsQueueIndex`)) (`self.TargetsQueueIndex`)) ; Event caught by BP_AbilityBase
            (`/Game/OldOnes/Core/Tools/BPFL_WidgetUtilities.Display Message to User` "") ; Hide text
            (else
              (bind _text (`self.InvestigableTargetsText` (`self.NumberOfTargetsToGet`) (`self.AreTargetsUnique`))) ; More Targets to get
              (`/Game/OldOnes/Core/Tools/BPFL_WidgetUtilities.Display Message to User` _text)))))
      (else
        (`/Game/OldOnes/Core/Tools/BPFL_WidgetUtilities.Display Message to User` "Investigable Already selected, please get another Target")))
    (else
      (goto _label))))

(fn `SelfCardHandler`
  (params (QueueIndex :type Integer))
  (bind (_returnvalue _viewedcard) (`/Game/OldOnes/Core/Tools/BPFL_GeneralFunctions.CardBeingPlayed`))
  (if _returnvalue
    (`self.SetTargetQueueTargetsAtIndex` QueueIndex (`|MakeArray` _viewedcard :!type "Object Object Reference"))
    (else
      (`KismetSystemLibrary.PrintString` "BP_AbilityTargetingManager::SelfCardHandler: Card trying to target self yet there is no card being played"))))

(fn `SelfEnemyHandler`
  (params (QueueIndex :type Integer))
  (bind _asbp_enemy (cast `/Game/OldOnes/Core/Enemy/BP_Enemy` (`/Game/OldOnes/Core/Tools/BPFL_GeneralFunctions.Get Active Character`))
    (:`then`
      (`self.SetTargetQueueTargetsAtIndex` QueueIndex (`|MakeArray` _asbp_enemy :!type "Object Object Reference")))
    (:`CastFailed`
      (`KismetSystemLibrary.PrintString` "BP_AbilityTargetingManager::SelfEnemyHandler: Trying to target self yet the active character is not an Enemy"))))

(fn `SelfTargetingHandler`
  (params (TargetsTags :type "Array of /Game/OldOnes/Core/Abilities/SAbilityAttribute Structure") (QueueIndex :type Integer))
  (bind _queueindex (`local.QueueIndex`))
  (if (`/Game/OldOnes/Core/Abilities/BPFL_AbilityAttributeParser.HasTag` TargetsTags (struct :`TagName` "TargetingStyle.Card.Self"))
    (`self.SelfCardHandler` _queueindex)
    (elif (`/Game/OldOnes/Core/Abilities/BPFL_AbilityAttributeParser.HasTag` TargetsTags (struct :`TagName` "TargetingStyle.Enemy.Self"))
      (`self.SelfEnemyHandler` _queueindex)
      (else
        (`KismetSystemLibrary.PrintString` "BP_AbilityTargetingManager::SelfTargetingHandler: Target Type not handled" true true (struct :`A` 1.0) 20.0)))))

(fn `SetTargetQueueTargetsAtIndex`
  (params (Index :type Integer) (Targets :type "Array of Object Object Reference"))
  (bind _stargetsarray (make `/Game/OldOnes/Core/Abilities/STargetsArray` Targets))
  (`KismetArrayLibrary.Array_Set` (`self.TargetsQueue`) Index _stargetsarray true)
  (`self.TargetingDoneEvent` _stargetsarray Index))

(fn `SpecificCardHandler`
  (params (TargetsTags :type "Array of /Game/OldOnes/Core/Abilities/SAbilityAttribute Structure") (NumberOfTargets :type Integer) (QueueIndex :type Integer))
  (set `self.TargetsQueueIndex` QueueIndex)
  (bind _foundcards (`/Game/OldOnes/Core/Tools/BPFL_Cards.FindCardsFromAbilityStruct` TargetsTags))
  (bind _selectableviews (`/Game/OldOnes/Core/PlayerUI/WBP_GameUI.MakeCardSelectionFromSearchResults` (`/Game/OldOnes/Core/Tools/BPFL_GeneralFunctions.GetPlayerUI`) _foundcards))
  (bind _output_get (set `self.SelectableCards` _selectableviews))
  (`self.TargetSpecificCards` (`local.NumberOfTargets`) _output_get (not (`/Game/OldOnes/Core/Abilities/BPFL_AbilityAttributeParser.HasTag` (`local.TargetsTags`) (struct :`TagName` "TargetRestriction.RepeatableTargets")))))

(fn `SpecificEnemyHandler`
  (params (TargetsTags :type "Array of /Game/OldOnes/Core/Abilities/SAbilityAttribute Structure") (NumberOfTargets :type Integer) (QueueIndex :type Integer))
  (set `self.TargetsQueueIndex` QueueIndex)
  (`self.TargetSpecificEnemies` NumberOfTargets (not (`/Game/OldOnes/Core/Abilities/BPFL_AbilityAttributeParser.HasTag` TargetsTags (struct :`TagName` "TargetRestriction.RepeatableTargets")))))

(fn `SpecificInvestigableHandler`
  (params (TargetsTags :type "Array of /Game/OldOnes/Core/Abilities/SAbilityAttribute Structure") (NumberOfTargets :type Integer) (QueueIndex :type Integer))
  (set `self.TargetsQueueIndex` QueueIndex)
  (`self.TargetSpecificInvestigables` NumberOfTargets (not (`/Game/OldOnes/Core/Abilities/BPFL_AbilityAttributeParser.HasTag` TargetsTags (struct :`TagName` "TargetRestriction.RepeatableTargets")))))

(fn `SpecificTargetsHandler`
  (params (TargetsTags :type "Array of /Game/OldOnes/Core/Abilities/SAbilityAttribute Structure") (QueueIndex :type Integer))
  (bind (_hastag _tagattributevalue) (`/Game/OldOnes/Core/Abilities/BPFL_AbilityAttributeParser.HasTag` TargetsTags (struct :`TagName` "TargetingStyle.Enemy")))
  (bind (_hastag_2 _tagattributevalue_2) (`/Game/OldOnes/Core/Abilities/BPFL_AbilityAttributeParser.HasTag` TargetsTags (struct :`TagName` "TargetingStyle.Investigable")))
  (bind (_hastag_3 _tagattributevalue_3) (`/Game/OldOnes/Core/Abilities/BPFL_AbilityAttributeParser.HasTag` TargetsTags (struct :`TagName` "TargetingStyle.Card")))
  (bind _queueindex (`local.QueueIndex`))
  (bind _targetstags (`local.TargetsTags`))
  (if _hastag_3
    (`self.SpecificCardHandler` _targetstags _tagattributevalue_3 _queueindex)
    (elif _hastag
      (`self.SpecificEnemyHandler` _targetstags _tagattributevalue _queueindex)
      (elif _hastag_2
        (`self.SpecificInvestigableHandler` _targetstags _tagattributevalue_2 _queueindex)
        (else
          (`KismetSystemLibrary.PrintString` "BP_AbilityTargetingManager::SpecifcTargetHandler: Type of object targetable not supported" true true (struct :`G` 0.66 :`B` 1.0 :`A` 1.0) 10.0))))))

(fn `TargetSpecificCards`
  (params (NumberOfCards :type Integer) (CardViews :type "Array of /Game/OldOnes/Core/PlayerUI/WBP_CardView Object Reference") (TargetsUnique :type Boolean))
  (bind _returnvalue (`KismetArrayLibrary.Array_Length` CardViews))
  (bind _numberofcards (`local.NumberOfCards`))
  ;[1 1 1] Setup Ability Targeting Object settings for the specific targeting
  (if (> _returnvalue 0)
    (bind _output_get (set `self.AreTargetsUnique` (`local.TargetsUnique`)))
    (if _output_get
      (set `self.NumberOfTargetsToGet` (`KismetMathLibrary.Min` _returnvalue _numberofcards))
      (else
        (set `self.NumberOfTargetsToGet` _numberofcards)))
    (`KismetArrayLibrary.Array_Set` (`self.TargetsQueue`) (`self.TargetsQueueIndex`) (make `/Game/OldOnes/Core/Abilities/STargetsArray` _) true)
    ;[1 1 1] Toggle cards selectability and bind self to the events of a card being selected
    (for _array_element (`local.CardViews`)
      (`/Game/OldOnes/Core/PlayerUI/WBP_CardView.ToggleTargetable` _array_element true)
      (add `/Game/OldOnes/Core/PlayerUI/WBP_CardView.CardTargetedEvent` _array_element (`|CreateDelegate` :!event `ReceiveCardTargetedEvent`)))
    (bind _text (`self.CardsTargetsText` (`self.NumberOfTargetsToGet`) (`self.AreTargetsUnique`)))
    (`/Game/OldOnes/Core/Tools/BPFL_WidgetUtilities.Display Message to User` _text)
    (else
      (`KismetSystemLibrary.PrintString` "BP_AbilityTargetingManager::TargetSpecificCards called with no cards selectable"))))

(fn `TargetSpecificEnemies`
  (params (NumberTargets :type Integer) (TargetsUnique :type Boolean :default true))
  (locals (Different :type Text) (Ennemies :type Text))
  (bind _numbertargets (`local.NumberTargets`))
  (bind _enemies (`/Game/OldOnes/Core/Tools/BPFL_Targeting.GetAllEnemies`))
  (bind _returnvalue (`KismetArrayLibrary.Array_Length` _enemies))
  (if (> _returnvalue 0)
    (bind _output_get (set `self.AreTargetsUnique` (`local.TargetsUnique`)))
    (if _output_get
      (set `self.NumberOfTargetsToGet` (`KismetMathLibrary.Min` _returnvalue _numbertargets))
      (else
        (set `self.NumberOfTargetsToGet` _numbertargets)))
    (`KismetArrayLibrary.Array_Set` (`self.TargetsQueue`) (`self.TargetsQueueIndex`) (make `/Game/OldOnes/Core/Abilities/STargetsArray` _) true)
    (add `/Game/OldOnes/Core/Player/BP_CardPlayerController.EnemyClickedEvent` (`/Game/OldOnes/Core/Tools/BPFL_GeneralFunctions.GetCardPlayerController`) (`|CreateDelegate` :!event `Receive Enemy Clicked Event`))
    (bind _text (`self.EnemyTargetsText` (`self.NumberOfTargetsToGet`) (`self.AreTargetsUnique`)))
    (`/Game/OldOnes/Core/Tools/BPFL_WidgetUtilities.Display Message to User` _text)
    (else
      (`KismetSystemLibrary.PrintString` "BP_AbilityTargetingManager::TargetSpecificEnemies called with no enemies on the board"))))

(fn `TargetSpecificInvestigables`
  (params (NumberOfInvestigables :type Integer) (TargetsUnique :type Boolean))
  (locals (NewLocalVar_0 :type "/Game/OldOnes/Core/Abilities/STargetsArray Structure"))
  (bind _numberofinvestigables (`local.NumberOfInvestigables`))
  (if (> (`KismetArrayLibrary.Array_Length` (`/Game/OldOnes/Core/GameSettings/BP_CardMode.Investigables` (`/Game/OldOnes/Core/Tools/BPFL_GeneralFunctions.GetCardGameMode`))) 0)
    (bind _output_get (set `self.AreTargetsUnique` (`local.TargetsUnique`)))
    (if _output_get
      (set `self.NumberOfTargetsToGet` (`KismetMathLibrary.Min` 0 _numberofinvestigables))
      (else
        (set `self.NumberOfTargetsToGet` _numberofinvestigables)))
    (`KismetArrayLibrary.Array_Set` (`self.TargetsQueue`) (`self.TargetsQueueIndex`) (make `/Game/OldOnes/Core/Abilities/STargetsArray` _) true)
    (add `/Game/OldOnes/Core/Player/BP_CardPlayerController.InvestigableClickedEvent` (`/Game/OldOnes/Core/Tools/BPFL_GeneralFunctions.GetCardPlayerController`) (`|CreateDelegate` :!event `ReceiveInvestigableClickedEvent`))
    (bind _text (`self.InvestigableTargetsText` (`self.NumberOfTargetsToGet`) (`self.AreTargetsUnique`)))
    (`/Game/OldOnes/Core/Tools/BPFL_WidgetUtilities.Display Message to User` _text)
    (else
      (`KismetSystemLibrary.PrintString` "BP_AbilityTargetingManager::TargetSpecificInvestigable: called with no Investigable on the board"))))