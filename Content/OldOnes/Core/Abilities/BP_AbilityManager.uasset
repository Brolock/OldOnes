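; BP_AbilityManager manages the set of abilities on its owning actor, covering playability checks, targeting, execution and ability text.
; Each ability is added as a component built from a struct holding its class and attributes, and can be packed back into structs.
; GetTargets starts targeting on all abilities without waiting; per-index done callbacks fill a flag array and fire TargetsReadyForExecution once all are set.
; ExecuteAbilities resets those flags, then executes every ability.
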(fn `AddAbilities`
  (params (AbilitiesAbstractStruct :type "Array of /Game/OldOnes/Core/Abilities/SAbilityAbstract Structure"))
  (for _array_element AbilitiesAbstractStruct
    (`self.AddAbility` _array_element)))

(fn `AddAbility`
  (params (AbilityAbstractStruct :type "/Game/OldOnes/Core/Abilities/SAbilityAbstract Structure"))
  (bind (_ability _abilityattributes) (break `/Game/OldOnes/Core/Abilities/SAbilityAbstract` AbilityAbstractStruct))
  (bind _returnvalue (`|AddComponentByClass` (`self.GetOwner`) _ability _abilityattributes (`KismetArrayLibrary.Array_Length` (`self.Abilities`))))
  (add `/Game/OldOnes/Core/Abilities/BP_AbilityInterface.TargetingDoneEvent` _returnvalue (`|CreateDelegate` :!event `SingleAbilityTargetingDone`))
  (`KismetArrayLibrary.Array_Add` (`self.Abilities`) _returnvalue)
  (`KismetArrayLibrary.Array_Add` (`self.AbilitiesForWhichTargetingIsDone`)))

(fn `CheckPlayability`
  (returns (Playable :type Boolean) (PlayabilityText :type Text))
  (for _array_element (`self.Abilities`)
    (bind (_playable _playabilitytext) (`/Game/OldOnes/Core/Abilities/BP_AbilityInterface.CheckPlayability` _array_element))
    (if (not _playable)
      (return false _playabilitytext)))
  (return true ""))

(fn `ExecuteAbilities`
  (for (_ _array_index) (`self.AbilitiesForWhichTargetingIsDone`)
    (`KismetArrayLibrary.Array_Set` (`self.AbilitiesForWhichTargetingIsDone`) _array_index) ; Reset for next Targeting session
  )
  (for _array_element (`self.Abilities`)
    (`/Game/OldOnes/Core/Abilities/BP_AbilityInterface.Execute` _array_element)))

(fn `GetAbilitiesText`
  (returns (AbilitiesText :type "Array of Text"))
  (locals (AbilitiesTextLocal :type "Array of Text"))
  (for _array_element (`self.Abilities`)
    (`KismetArrayLibrary.Array_Add` (`local.AbilitiesTextLocal`) (`/Game/OldOnes/Core/Abilities/BP_AbilityInterface.Get Ability Text` _array_element)))
  (return (`local.AbilitiesTextLocal`)))

(fn `GetTargets`
  (for _array_element (`self.Abilities`)
    (`/Game/OldOnes/Core/Abilities/BP_AbilityInterface.GetAbilityTargets` _array_element) ; How do I wait for the targets of this ability to be done here SEND HELP
  ))

(fn `PackAbilitiesToStruct`
  (returns (AbilityStructs :type "Array of /Game/OldOnes/Core/Abilities/SAbilityAbstract Structure"))
  (locals (LocalAbilityStructs :type "Array of /Game/OldOnes/Core/Abilities/SAbilityAbstract Structure"))
  (for _array_element (`self.Abilities`)
    (bind _abilitystruct (`/Game/OldOnes/Core/Abilities/BP_AbilityInterface.PackAbilityToStruct` _array_element))
    (`KismetArrayLibrary.Array_Add` (`local.LocalAbilityStructs`) _abilitystruct))
  (return (`local.LocalAbilityStructs`)))

(fn `SingleAbilityTargetingDone`
  (params (AbilityIndex :type Integer))
  (locals (AllTargetingDone :type Boolean :default true))
  (`KismetArrayLibrary.Array_Set` (`self.AbilitiesForWhichTargetingIsDone`) AbilityIndex true true)
  (for _array_element (`self.AbilitiesForWhichTargetingIsDone`)
    (if (not _array_element)
      (set `local.AllTargetingDone` false)))
  (if (`local.AllTargetingDone`)
    (`self.TargetsReadyForExecution`)))