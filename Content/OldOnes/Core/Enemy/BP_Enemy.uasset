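; BP_Enemy is a turn-based card-game enemy whose mesh, stats, animations and abilities come from a data asset during construction.
; It shuffles abilities and readies the first, acquires targets on turn start, then executes and ends its turn.
; Attacks with animations wait for an ExecuteAbility call, with a Tick timeout as fallback.
; It also plays idle, hit and death animations, ragdolling without a death clip, and turns its UI toward the camera.
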(event `self.ReceiveBeginPlay`
  (bind _aswbp_enemy_ui (cast `/Game/OldOnes/Core/Enemy/WBP_EnemyUI` (`WidgetComponent.GetUserWidgetObject` (`self.Widget`))))
  (`self.TurnEnemyTowardsPlayer`)
  (`/Game/OldOnes/Core/Enemy/WBP_EnemyUI.InitializeWidget` _aswbp_enemy_ui self)
  (set `self.MaximumAnimationDelay` (`/Game/OldOnes/Core/GameSettings/GameSettings_DataAsset.MaximumAnimationDelay` (`/Game/OldOnes/Core/Tools/BPFL_GeneralFunctions.GetGameSettingsDataAsset`))))

(event `self.ReceiveTick`
  (params (DeltaSeconds :type "Float (single-precision)"))
  (`self.TurnWidgetTowardsCamera`)
  (`self.WaitBeforeAbilityExecution` DeltaSeconds)
  ;[1 0 0.008603] Dirty way of playing idle animation while waiting for proper animation system
  (if (and (not (`SkeletalMeshComponent.IsPlaying` (`self.SkeletalMesh`))) (`self.IsAlive`))
    (`SkeletalMeshComponent.PlayAnimation` (`self.SkeletalMesh`) (`/Game/OldOnes/Core/Tools/BPFL_GeneralFunctions.GetAnimationFromDict` "NewEnumerator0" (`/Game/OldOnes/Core/Enemy/Enemy_DataAsset.GetAnimations` (`self.DataAsset`))) true)))

(event `AbilityTargetsAcquired`
  (params (FiringAbility :type "/Game/OldOnes/Core/Abilities/BP_AbilityManager Object Reference"))
  (bind (_softanimationsequence _animation_found) (`/Game/OldOnes/Core/Tools/BPFL_GeneralFunctions.GetAnimationFromDict` "NewEnumerator1" (`/Game/OldOnes/Core/Enemy/Enemy_DataAsset.GetAnimations` (`self.DataAsset`))))
  (set `self.IsWaitingForAnimationToExecute` true)
  (set `self.WaitingTime` 0.0)
  (switch `/Game/OldOnes/Core/Enemy/EEnemyActions` (`/Game/OldOnes/Core/Abilities/BP_AbilityManager.GetAbilityType` FiringAbility)
    (:`NewEnumerator0`
      (if _animation_found
        (`SkeletalMeshComponent.PlayAnimation` (`self.SkeletalMesh`) _softanimationsequence false)
        (else
          (`self.ExecuteAbility`))))
    (:`NewEnumerator1`
      (`self.ExecuteAbility`))))

(fn `Destroy_GameReset`
  (bind _widget (`self.Widget`))
  (`Widget.SetVisibility` (`WidgetComponent.GetWidget` _widget) "Collapsed")
  (`ActorComponent.K2_DestroyComponent` _widget)
  (`self.SetActorHiddenInGame` true)
  (for _array_element (`self.EnemyAbilities`)
    (`ActorComponent.K2_DestroyComponent` _array_element))
  (`self.K2_DestroyActor`))

(fn `Die`
  (bind (_softanimationsequence _animation_found) (`/Game/OldOnes/Core/Tools/BPFL_GeneralFunctions.GetAnimationFromDict` "NewEnumerator3" (`/Game/OldOnes/Core/Enemy/Enemy_DataAsset.GetAnimations` (`self.DataAsset`))))
  (`parent.Die`)
  (set `self.IsAlive` false)
  (`SceneComponent.SetVisibility` (`self.Widget`) false true)
  (if _animation_found
    (`SkeletalMeshComponent.PlayAnimation` (`self.SkeletalMesh`) _softanimationsequence false)
    (else
      (`PrimitiveComponent.SetSimulatePhysics` (`self.SkeletalMesh`) true))))

(fn `EndGame`
  (`parent.EndGame`))

(fn `EndTurn`
  (if (`self.IsAlive`)
    (`parent.EndTurn`)
    (`self.CharacterEndTurnEvent` self)))

(fn `ExecuteAbility`
  (if (`self.IsWaitingForAnimationToExecute`)
    (set `self.IsWaitingForAnimationToExecute` false)
    (`/Game/OldOnes/Core/Abilities/BP_AbilityManager.ExecuteAbilities` (`|GetArrayItem` (`self.EnemyAbilities`)))
    (`KismetArrayLibrary.Array_Shuffle` (`self.EnemyAbilities`))
    (`self.ReadyingAbility` (`|GetArrayItem` (`self.EnemyAbilities`)))
    (`self.EndTurn`)
    (else
      (`KismetSystemLibrary.PrintString` "BP_Enemy::ExecuteAbility received while not waiting for execution through animation. Do not call this function outside of the normal loop of execution" true true (struct :`R` 1.0 :`A` 1.0) 30.0))))

(fn `InitializeEnemy`
  (bind _enemyabilities (`self.EnemyAbilities`))
  (bind _skeletalmesh (`self.SkeletalMesh`))
  (bind _dataasset (`self.DataAsset`))
  (bind _dataasset_2 (`self.DataAsset`))
  (`SkinnedMeshComponent.SetSkinnedAssetAndUpdate` _skeletalmesh (`/Game/OldOnes/Core/Enemy/Enemy_DataAsset.GetSkeletalMesh` _dataasset_2) true)
  (`SkeletalMeshComponent.OverrideAnimationData` _skeletalmesh (`/Game/OldOnes/Core/Tools/BPFL_GeneralFunctions.GetAnimationFromDict` "NewEnumerator0" (`/Game/OldOnes/Core/Enemy/Enemy_DataAsset.GetAnimations` _dataasset_2)) true true 0.0 1.0)
  ;[1 1 1] Initialize base stats
  (set `self.CurrentHP` (`/Game/OldOnes/Core/Enemy/Enemy_DataAsset.StartingHP` _dataasset))
  (set `self.MaxHP` (`/Game/OldOnes/Core/Enemy/Enemy_DataAsset.MaxHP` _dataasset))
  (set `self.Block` (`/Game/OldOnes/Core/Enemy/Enemy_DataAsset.StartingBlock` _dataasset))
  ;[1 1 1] Initialize Abilities
  (for _array_element (`/Game/OldOnes/Core/Enemy/Enemy_DataAsset.Abilities` (`self.DataAsset`))
    (bind _returnvalue (`|AddComponentByClass` "/Game/OldOnes/Core/Abilities/BP_AbilityManager.BP_AbilityManager_C"))
    (bind _returnvalue_2 (`KismetArrayLibrary.Array_Add` _enemyabilities _returnvalue))
    (`/Game/OldOnes/Core/Abilities/BP_AbilityManager.AddAbilities` (`|GetArrayItem` _enemyabilities _returnvalue_2) (`.AbilityEffects_3_015077CB4D0FE6608B462F818CE2A719` (break `/Game/OldOnes/Core/Enemy/SEnemyAbilities` _array_element)))
    (add `/Game/OldOnes/Core/Abilities/BP_AbilityManager.TargetsReadyForExecution` _returnvalue (`|CreateDelegate` :!event `AbilityTargetsAcquired`))))

(fn `StartGame`
  (`parent.StartGame`)
  (`KismetArrayLibrary.Array_Shuffle` (`self.EnemyAbilities`))
  (`self.ReadyingAbility` (`|GetArrayItem` (`self.EnemyAbilities`))))

(fn `StartTurn`
  (`parent.StartTurn`)
  (`/Game/OldOnes/Core/Abilities/BP_AbilityManager.GetTargets` (`|GetArrayItem` (`self.EnemyAbilities`))))

(fn `TakeDamage`
  (params (AmountToTake :type Integer))
  (returns (DamageTaken :type Integer) (BlockTaken :type Integer))
  (bind (_softanimationsequence _animation_found) (`/Game/OldOnes/Core/Tools/BPFL_GeneralFunctions.GetAnimationFromDict` "NewEnumerator2" (`/Game/OldOnes/Core/Enemy/Enemy_DataAsset.GetAnimations` (`self.DataAsset`))))
  (if _animation_found
    (`SkeletalMeshComponent.PlayAnimation` (`self.SkeletalMesh`) _softanimationsequence false))
  (bind (_damagetaken _blocktaken) (`parent.TakeDamage` AmountToTake))
  (return _damagetaken _blocktaken))

(fn `TurnEnemyTowardsPlayer`
  (locals (ActorToTurnTowards :type "Actor Object Reference"))
  (bind _player3dmodel (`/Game/OldOnes/Core/GameSettings/BP_CardMode.Player3DModel` (`/Game/OldOnes/Core/Tools/BPFL_GeneralFunctions.GetCardGameMode`)))
  (bind (_returnvalue_roll _returnvalue_pitch _returnvalue_yaw) (`KismetMathLibrary.BreakRotator` (`KismetMathLibrary.FindLookAtRotation` (`self.K2_GetActorLocation`) (`self.K2_GetActorLocation` (`local.ActorToTurnTowards`)))))
  (`/Engine/EditorBlueprintResources/StandardMacros.IsValid` _player3dmodel
    (:`Is Valid`
      (set `local.ActorToTurnTowards` _player3dmodel))
    (:`Is Not Valid`
      (set `local.ActorToTurnTowards` (`/Game/OldOnes/Core/Tools/BPFL_GeneralFunctions.GetCardPlayerPawn`))))
  (`self.K2_SetActorRotation` (`KismetMathLibrary.MakeRotator` 0.0 0.0 _returnvalue_yaw) true)
  (set `self.PlayerGameraRef` (`/Game/OldOnes/Core/Tools/BPFL_GeneralFunctions.GetPlayerCamera`)) ; Keep camera in reference to turn UI torwards it
)

(fn `TurnWidgetTowardsCamera`
  (`SceneComponent.K2_SetWorldRotation` (`self.Widget`) (`KismetMathLibrary.FindLookAtRotation` (`SceneComponent.K2_GetComponentLocation` (`self.Widget`)) (`SceneComponent.K2_GetComponentLocation` (`self.PlayerGameraRef`))) false false))

(fn `UserConstructionScript`
  (bind _widget (`self.Widget`))
  (`/Engine/EditorBlueprintResources/StandardMacros.IsValid` (`self.DataAsset`)
    (:`Is Valid`
      (`self.InitializeEnemy`)
      (`SceneComponent.SetRelativeScale3D` _widget (* (`SceneComponent.RelativeScale3D` _widget) (/ (1.0 1.0 1.0) (`SceneComponent.K2_GetComponentScale` (`self.DefaultSceneRoot`))))))))

(fn `WaitBeforeAbilityExecution`
  (params (DeltaTime :type "Float (double-precision)"))
  (if (`self.IsWaitingForAnimationToExecute`)
    (bind _output_get (set `self.WaitingTime` (+ (`self.WaitingTime`) DeltaTime)))
    (if (>= _output_get (`self.MaximumAnimationDelay`))
      (`self.ExecuteAbility`))))