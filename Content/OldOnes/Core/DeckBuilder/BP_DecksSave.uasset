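; BP_DecksSave stores the deck builder's decks in a SavedDecks map keyed by deck name.
; AddDeckToSave packs a deck's cards into struct form and passes them to AddDeckStructToSavedDecks, which wraps them in an SDeckSave entry and adds it to the map.
; An empty name prints a warning and falls back to "DefaultName".
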(fn `AddDeckStructToSavedDecks`
  (params (DeckCards :type "Array of /Game/OldOnes/Core/Cards/SCardData Structure") (DeckName :type String))
  (locals (LocalDeckName :type String))
  (set `local.LocalDeckName` DeckName)
  (if (`KismetStringLibrary.IsEmpty` DeckName)
    (`KismetSystemLibrary.PrintString` null "AddDeckToSave: DeckName empty, please chose a deck name. Using DefaultName instead" true true (struct :`R` 1.0 :`G` 0.068094 :`A` 1.0) 30.0)
    (set `local.LocalDeckName` "DefaultName"))
  (`BlueprintMapLibrary.Map_Add` (`self.SavedDecks`) (`local.LocalDeckName`) (make `/Game/OldOnes/Core/DeckBuilder/SDeckSave` (`local.DeckCards`))))

(fn `AddDeckToSave`
  (params (Deck :type "/Game/OldOnes/Core/CardPile/BP_CardPile Object Reference") (DeckName :type String))
  (locals (GeneratedDeckIdx :type Integer) (DeckNameLocal :type String))
  (bind _cardsstruct (`/Game/OldOnes/Core/CardPile/BP_CardPile.PackCardsToStruct` Deck))
  (`self.AddDeckStructToSavedDecks` _cardsstruct DeckName))