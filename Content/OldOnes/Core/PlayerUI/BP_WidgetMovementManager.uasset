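; BP_WidgetMovementManager animates player UI widgets by easing their render transforms from start to destination.
; AddMovementStruct queues movements in a map keyed by widget name, optionally staggering them with negative starting alpha from an accumulating delay.
; MoveWidgets decays that delay, advances each alpha, applies expo-out easing to translation, scale, shear and angle, then removes finished entries.
; Helpers compare transforms within tolerances and report whether widgets are queued or moving.
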(fn `Add Movement Struct`
  (params (WidgetInterpolationStruct :type "/Game/OldOnes/Core/PlayerUI/SWidgetInterpolationTuple Structure") (NoDelayOnAnimation :type Boolean))
  (bind (_widget _start _destination _alpha _speed _modifier) (break `/Game/OldOnes/Core/PlayerUI/SWidgetInterpolationTuple` WidgetInterpolationStruct))
  (bind (_widget_2 _start_2 _destination_2 _alpha_2 _speed_2 _modifier_2) (break `/Game/OldOnes/Core/PlayerUI/SWidgetInterpolationTuple` WidgetInterpolationStruct))
  (if NoDelayOnAnimation
    (`BlueprintMapLibrary.Map_Add` (`self.WidgetToInterpolationStruct`) (`KismetSystemLibrary.GetObjectName` _widget_2) (make `/Game/OldOnes/Core/PlayerUI/SWidgetInterpolationTuple` _widget_2 _start_2 _destination_2 _alpha_2 _speed_2 _modifier_2))
    (else
      (`BlueprintMapLibrary.Map_Add` (`self.WidgetToInterpolationStruct`) (`KismetSystemLibrary.GetObjectName` _widget) (make `/Game/OldOnes/Core/PlayerUI/SWidgetInterpolationTuple` _widget _start _destination (- _alpha (`self.AnimationDelay`)) _speed _modifier))
      (set `self.AnimationDelay` (+ (`self.AnimationDelay`) (`self.DeltaTimeBetweenAnimations`))))))

(fn `AreWidgetsTransformEqual`
  (params (First :type "WidgetTransform Structure") (Second :type "WidgetTransform Structure") (PositionalTolerance :type "Float (double-precision)") (AngleTolerance :type "Float (double-precision)"))
  (returns (TransformsEquals :type Boolean))
  (bind (_translation _scale _shear _angle) (break `WidgetTransform` First))
  (bind (_translation_2 _scale_2 _shear_2 _angle_2) (break `WidgetTransform` Second))
  (bind _positionaltolerance (`local.PositionalTolerance`))
  (return (and (== _translation _translation_2 :`ErrorTolerance` _positionaltolerance) (== _scale _scale_2 :`ErrorTolerance` _positionaltolerance) (== _shear _shear_2 :`ErrorTolerance` _positionaltolerance) (`KismetMathLibrary.NearlyEqual_FloatFloat` _angle _angle_2 AngleTolerance))))

(fn `IsWidgetInAnimationQueue`
  (params (Widget :type "Widget Object Reference"))
  (returns (IsQueued :type Boolean))
  (return (`BlueprintMapLibrary.Map_Contains` (`self.WidgetToInterpolationStruct`) (`KismetSystemLibrary.GetObjectName` Widget))))

(fn `IsWidgetMoving`
  (params (Widget :type "Widget Object Reference"))
  (returns (IsMoving :type Boolean))
  (bind (_value _returnvalue) (`BlueprintMapLibrary.Map_Find` (`self.WidgetToInterpolationStruct`) (`KismetSystemLibrary.GetObjectName` Widget)))
  (return (and _returnvalue (>= (`.Alpha_10_7C7080774750A0A4D401CBACCC6E5AF5` (break `/Game/OldOnes/Core/PlayerUI/SWidgetInterpolationTuple` _value)) 0.0))))

(fn `MoveWidgets`
  (params (DeltaTime :type "Float (double-precision)" :default 0.0))
  (locals (AnimationDoneWidgets :type "Array of String"))
  (set `self.AnimationDelay` (`KismetMathLibrary.FClamp` (- (`self.AnimationDelay`) DeltaTime) 0.0 (`self.MaximumDelay`)))
  (bind _values (`BlueprintMapLibrary.Map_Values` (`self.WidgetToInterpolationStruct`)))
  (for _array_element _values
    (bind (_widget _start _destination _alpha _speed _modifier) (break `/Game/OldOnes/Core/PlayerUI/SWidgetInterpolationTuple` _array_element))
    (`/Engine/EditorBlueprintResources/StandardMacros.IsValid` _widget
      (:`Is Valid`
        (bind _swidgetinterpolationtuple (make `/Game/OldOnes/Core/PlayerUI/SWidgetInterpolationTuple` _widget _start _destination (+ _alpha (* _speed (`local.DeltaTime`) (`self.SpeedModifier`))) _speed _modifier))
        (`BlueprintMapLibrary.Map_Add` (`self.WidgetToInterpolationStruct`) (`KismetSystemLibrary.GetObjectName` _widget) _swidgetinterpolationtuple) ; BP_Maps are Immutable we have to re-add the element
        (bind (_widget_2 _start_2 _destination_2 _alpha_2 _speed_2 _modifier_2) (break `/Game/OldOnes/Core/PlayerUI/SWidgetInterpolationTuple` _swidgetinterpolationtuple))
        (if (>= _alpha_2 0.0)
          (bind _interpolatedwidget (`self.WidgetTransformEase` _start_2 _destination_2 _alpha_2 _modifier_2 "ExpoOut" :!pinned true)) ; Chose interpolation here
          (`Widget.SetRenderTransform` _widget_2 _interpolatedwidget)
          (if (> _alpha_2 1.0)
            (`KismetArrayLibrary.Array_Add` (`local.AnimationDoneWidgets`) (`KismetSystemLibrary.GetObjectName` _widget_2)))))
      (:`Is Not Valid`
        (`KismetSystemLibrary.PrintString` null "WidgetMovementManger::MoveWidgetsToTheirDestination: Widget has movement but has been deleted" true true (struct :`R` 1.0 :`G` 0.197471 :`A` 1.0)) ; This case should never happen but if it does handle the case by removing it from the map
      )))
  (for _array_element_2 (`local.AnimationDoneWidgets`)
    (`BlueprintMapLibrary.Map_Remove` (`self.WidgetToInterpolationStruct`) _array_element_2)))

(fn `Remove Widget`
  (params (Widget :type "Widget Object Reference"))
  (`BlueprintMapLibrary.Map_Remove` (`self.WidgetToInterpolationStruct`) (`KismetSystemLibrary.GetObjectName` Widget)))

(fn `Vector2DEase`
  (params (Start :type "Vector2D Structure") (End :type "Vector2D Structure") (Alpha :type "Float (double-precision)") (InterpFunction :type "EEasingFunc Enum" :default "Linear") (Modifier :type "Float (double-precision)"))
  (returns (InterpolatedVector :type "Vector2D Structure"))
  (bind (_x _y) (`KismetMathLibrary.BreakVector2D` Start))
  (bind (_x_2 _y_2) (`KismetMathLibrary.BreakVector2D` End))
  (bind _alpha (`local.Alpha`))
  (bind _modifier (`local.Modifier`))
  (return (`KismetMathLibrary.MakeVector2D` (`|EaseFunction` InterpFunction _alpha _x _x_2 _modifier) (`|EaseFunction` InterpFunction _alpha _y _y_2 _modifier))))

(fn `WidgetTransformEase`
  (params (Start :type "WidgetTransform Structure") (End :type "WidgetTransform Structure") (Alpha :type "Float (double-precision)") (Modifier :type "Float (double-precision)") (InterpFunction :type "EEasingFunc Enum" :default "Linear"))
  (returns (InterpolatedWidget :type "WidgetTransform Structure"))
  (bind (_translation _scale _shear _angle) (break `WidgetTransform` Start))
  (bind (_translation_2 _scale_2 _shear_2 _angle_2) (break `WidgetTransform` End))
  (bind _modifier (`local.Modifier`))
  (bind _alpha (`local.Alpha`))
  (bind _interpfunction (`local.InterpFunction`))
  (bind _modifier_2 (`local.Modifier`))
  (bind _alpha_2 (`local.Alpha`))
  (bind _interpfunction_2 (`local.InterpFunction`))
  (return (make `WidgetTransform` (`self.Vector2DEase` _translation _translation_2 _alpha _interpfunction _modifier) (`self.Vector2DEase` _scale _scale_2 _alpha _interpfunction _modifier) (`self.Vector2DEase` _shear _shear_2 _alpha_2 _interpfunction_2 _modifier_2) (`|EaseFunction` _interpfunction_2 _alpha_2 _angle _angle_2 _modifier_2))))