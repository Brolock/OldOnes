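; BP_AbilitiesVerticalTextBlock is a vertical box UI element that shows a list of ability texts, styled with card UI settings.
; AddAbilityText creates a WBP_AbilityTextBlock child, applies the card font and color from the UI settings data asset, sets its text and gives it a Fill slot size.
; ResetAbilityTexts collapses and removes all children to clear the list.
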(fn `AddAbilityText`
  (params (AbilityText :type Text))
  (bind _uisettingdataasset (`/Game/OldOnes/Core/Tools/BPFL_GeneralFunctions.GetUISettingsDataAsset`))
  (bind _returnvalue (`|CreateWidget` "/Game/OldOnes/Core/PlayerUI/WBP_AbilityTextBlock.WBP_AbilityTextBlock_C"))
  (bind _returnvalue_2 (`self.AddChildToVerticalBox` _returnvalue))
  (bind _abilitytextblock (`/Game/OldOnes/Core/PlayerUI/WBP_AbilityTextBlock.AbilityTextBlock` _returnvalue))
  (`TextBlock.SetFont` _abilitytextblock (`/Game/OldOnes/Core/PlayerUI/UISetting_DataAsset.CardsFont` _uisettingdataasset))
  (`TextBlock.SetColorAndOpacity` _abilitytextblock (`/Game/OldOnes/Core/PlayerUI/UISetting_DataAsset.CardsFontColor` _uisettingdataasset))
  (`TextBlock.SetText` _abilitytextblock (`local.AbilityText`))
  (`VerticalBoxSlot.SetSize` _returnvalue_2 (make `SlateChildSize` 1.0)))

(fn `ResetAbilityTexts`
  (for _array_element (`self.GetAllChildren`)
    (`self.SetVisibility` _array_element "Collapsed")
    (`self.RemoveFromParent` _array_element)))