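; BP_HandManager manages the cards in a hand for the card game, holding them in a Cards array.
; It adds cards by changing their location to the hand, removes specific, random or all cards, and looks them up by index or type.
; Its fullness check makes an exception at exactly maximum size while a card is being played.
; It can also pack the hand into an array of card structs.
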(fn `AddCardToHand`
  (params (Card :type "/Game/OldOnes/Core/Cards/BP_Card Object Reference"))
  (`/Game/OldOnes/Core/Cards/BP_Card.ChangeLocation` Card (`self.HandLocation`))
  (`KismetArrayLibrary.Array_Add` (`self.Cards`) Card))

(fn `Get Cards Of Types`
  (params (CardTypes :type "Set of /Game/OldOnes/Core/Cards/ECardTypes Enum"))
  (returns (FoundCards :type "Array of /Game/OldOnes/Core/Cards/BP_Card Object Reference"))
  (locals (FoundCardsLocal :type "Array of /Game/OldOnes/Core/Cards/BP_Card Object Reference"))
  (for _array_element (`self.Cards`)
    (if (`BlueprintSetLibrary.Set_Contains` CardTypes (`/Game/OldOnes/Core/Cards/BP_Card.GetCardType` _array_element))
      (`KismetArrayLibrary.Array_Add` (`local.FoundCardsLocal`) _array_element)))
  (return (`local.FoundCardsLocal`)))

(fn `GetCardAtIndex`
  (params (Index :type Integer))
  (returns (Card :type "/Game/OldOnes/Core/Cards/BP_Card Object Reference"))
  (if (<= Index (`KismetArrayLibrary.Array_LastIndex` (`self.Cards`)))
    (return (`|GetArrayItem` (`self.Cards`) Index))
    (else
      (`KismetSystemLibrary.PrintString` "BP_HandManager::GetCardAtIndex: Trying to access a card at index higher of Cards array"))))

(fn `HandSize`
  (returns (HandSize :type Integer))
  (return (`KismetArrayLibrary.Array_Length` (`self.Cards`))))

(fn `IsHandFull`
  (returns (ReturnValue :type Boolean))
  (bind _maxhandsize (`self.MaxHandSize`))
  (bind _returnvalue (`KismetArrayLibrary.Array_Length` (`self.Cards`)))
  (if (and (`/Game/OldOnes/Core/Tools/BPFL_GeneralFunctions.CardBeingPlayed`) (== _returnvalue _maxhandsize))
    (return false)
    (elif (>= _returnvalue _maxhandsize)
      (return true))))

(fn `PackCardsToStruct`
  (returns (CardsStruct :type "Array of /Game/OldOnes/Core/Cards/SCardData Structure"))
  (locals (CardStructLocal :type "Array of /Game/OldOnes/Core/Cards/SCardData Structure"))
  (for _array_element (`self.Cards`)
    (`KismetArrayLibrary.Array_Add` (`local.CardStructLocal`) (`/Game/OldOnes/Core/Cards/BP_Card.PackCardToStruct` _array_element)))
  (return (`local.CardStructLocal`)))

(fn `RemoveAllCardsFromHand`
  (returns (RemovedCards :type "Array of /Game/OldOnes/Core/Cards/BP_Card Object Reference"))
  (locals (RemovedCardsLocal :type "Array of /Game/OldOnes/Core/Cards/BP_Card Object Reference"))
  (bind (_arrayindex _arrayelement) (`/Engine/EditorBlueprintResources/StandardMacros.ReverseForEachLoop` (`self.Cards`))
    (:`LoopBody`
      (bind _removedcard (`self.RemoveFromHand` _arrayelement))
      (`KismetArrayLibrary.Array_Add` (`local.RemovedCardsLocal`) _removedcard))
    (:`Completed`
      (return (`local.RemovedCardsLocal`)))))

(fn `RemoveFromHand`
  (params (Card :type "/Game/OldOnes/Core/Cards/BP_Card Object Reference"))
  (returns (RemovedCard :type "/Game/OldOnes/Core/Cards/BP_Card Object Reference") (WasSuccessful :type Boolean))
  (bind _returnvalue (`KismetArrayLibrary.Array_RemoveItem` (`self.Cards`) Card))
  (if _returnvalue
    (return Card true)
    (else
      (`KismetSystemLibrary.PrintString` "BP_HandManager::RemoveFromHand: Trying to  remove a card that is not in hand?" true true (struct :`G` 0.66 :`B` 1.0 :`A` 1.0) 20.0)
      (return null false))))

(fn `RemoveRandomCardFromHand`
  (returns (RemovedCard :type "/Game/OldOnes/Core/Cards/BP_Card Object Reference") (WasSuccessful :type Boolean))
  (bind (_removedcard _wassuccessful) (`self.RemoveFromHand` (`KismetArrayLibrary.Array_Random` (`self.Cards`))))
  (return _removedcard _wassuccessful))