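; BP_CardPile is an ordered card container that serves as a pile in a card game, with draw, shuffle, query and transfer operations.
; The array's last element is the top; added cards go top, bottom or random and update their location to the pile's type.
; Shuffling fires an event, and views are created per card in a container that, if a WBP_CardPIleView, binds to the pile's events.
; Helpers filter cards by type and pack them into structs.
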(fn `AddCardsToPile`
  (params (Cards :type "Array of /Game/OldOnes/Core/Cards/BP_Card Object Reference") (PilePosition :type "/Game/OldOnes/Core/CardPile/EPositionInPile Enum" :default "NewEnumerator0"))
  (for _array_element Cards
    (`self.AddCardToPile` _array_element PilePosition)))

(fn `AddCardToPile`
  (params (CardToAdd :type "/Game/OldOnes/Core/Cards/BP_Card Object Reference") (PilePosition :type "/Game/OldOnes/Core/CardPile/EPositionInPile Enum" :default "NewEnumerator0") (ShufflePile :type Boolean :default false))
  (bind _cardtoadd (`local.CardToAdd`))
  (bind _cards (`self.Cards`))
  (`/Game/OldOnes/Core/Cards/BP_Card.ChangeLocation` CardToAdd (`self.PileType`))
  (switch `/Game/OldOnes/Core/CardPile/EPositionInPile` PilePosition
    (:`NewEnumerator0`
      (`KismetArrayLibrary.Array_Add` _cards _cardtoadd))
    (:`NewEnumerator1`
      (`KismetArrayLibrary.Array_Insert` _cards _cardtoadd))
    (:`NewEnumerator2`
      (`KismetArrayLibrary.Array_Insert` _cards _cardtoadd (`KismetMathLibrary.RandomInteger` (`KismetArrayLibrary.Array_Length` (`self.Cards`))))))
  (if (`local.ShufflePile`)
    (`self.Shuffle`)))

(fn `BottomCard`
  (returns (Output :type "/Game/OldOnes/Core/Cards/BP_Card Object Reference"))
  (return (`|GetArrayItem` (`self.Cards`))))

(fn `ChangeCardsPile`
  (params (DestinationPile :type "/Game/OldOnes/Core/CardPile/BP_CardPile Object Reference"))
  (bind (_arrayindex _arrayelement) (`/Engine/EditorBlueprintResources/StandardMacros.ReverseForEachLoop` (`self.Cards`))
    (:`LoopBody`
      (bind _removedcard (`self.RemoveCardFromPile` _arrayelement))
      (`self.AddCardToPile` (`local.DestinationPile`) _removedcard "NewEnumerator0" false))))

(fn `DrawCard`
  (returns (CardDrawn :type "/Game/OldOnes/Core/Cards/BP_Card Object Reference") (CardValid :type Boolean))
  (bind (_removedcard _cardremoved) (`self.RemoveCardFromPile` (`self.TopCard`)))
  (return _removedcard _cardremoved))

(fn `GetCardsNames`
  (returns (CardsNames :type "Array of String"))
  (locals (CardsNamesLocal :type "Array of String"))
  (for _array_element (`self.Cards`)
    (`KismetArrayLibrary.Array_Add` (`local.CardsNamesLocal`) (`/Game/OldOnes/Core/Cards/BP_Card.GetName` _array_element)))
  (return (`local.CardsNamesLocal`)))

(fn `GetCardsOfTypes`
  (params (CardTypes :type "Set of /Game/OldOnes/Core/Cards/ECardTypes Enum"))
  (returns (CardsFound :type "Array of /Game/OldOnes/Core/Cards/BP_Card Object Reference"))
  (locals (CardsFoundLocal :type "Array of /Game/OldOnes/Core/Cards/BP_Card Object Reference"))
  (for _array_element (`self.Cards`)
    (if (`BlueprintSetLibrary.Set_Contains` CardTypes (`/Game/OldOnes/Core/Cards/BP_Card.GetCardType` _array_element))
      (`KismetArrayLibrary.Array_Add` (`local.CardsFoundLocal`) _array_element)))
  (return (`local.CardsFoundLocal`)))

(fn `GetNumberOfCards`
  (returns (NumberOfCards :type Integer))
  (return (`KismetArrayLibrary.Array_Length` (`self.Cards`))))

(fn `InitializeCardViews`
  (params (CardContainerView :type "/Game/OldOnes/Core/PlayerUI/WBP_CardContainerParent Object Reference"))
  (for _array_element (`self.Cards`)
    (bind _view (`/Game/OldOnes/Core/Tools/BPFL_Cards.CreateViewFromCard` _array_element))
    (`/Game/OldOnes/Core/PlayerUI/WBP_CardContainerParent.AddCardToContainer` CardContainerView _view null))
  (bind _aswbp_card_pile_view (cast `/Game/OldOnes/Core/PlayerUI/WBP_CardPIleView` (`local.CardContainerView`)))
  (`/Game/OldOnes/Core/PlayerUI/WBP_CardPIleView.Bind Events to Pile` _aswbp_card_pile_view self))

(fn `IsEmpty`
  (returns (DeckEmpty :type Boolean))
  (return (== (`KismetArrayLibrary.Array_Length` (`self.Cards`)) 0)))

(fn `PackCardsToStruct`
  (returns (CardsStruct :type "Array of /Game/OldOnes/Core/Cards/SCardData Structure"))
  (locals (CardsStructLocal :type "Array of /Game/OldOnes/Core/Cards/SCardData Structure"))
  (for _array_element (`self.Cards`)
    (`KismetArrayLibrary.Array_Add` (`local.CardsStructLocal`) (`/Game/OldOnes/Core/Cards/BP_Card.PackCardToStruct` _array_element)))
  (return (`local.CardsStructLocal`)))

(fn `RemoveCardFromPile`
  (params (Card :type "/Game/OldOnes/Core/Cards/BP_Card Object Reference"))
  (returns (RemovedCard :type "/Game/OldOnes/Core/Cards/BP_Card Object Reference") (CardRemoved :type Boolean))
  (bind _returnvalue (`KismetArrayLibrary.Array_RemoveItem` (`self.Cards`) Card))
  (if _returnvalue
    (return Card _returnvalue)
    (else
      (return null false))))

(fn `Shuffle`
  (`KismetArrayLibrary.Array_Shuffle` (`self.Cards`))
  (`self.ShuffleDeckEvent`))

(fn `TopCard`
  (returns (Output :type "/Game/OldOnes/Core/Cards/BP_Card Object Reference"))
  (bind _cards (`self.Cards`))
  (return (`|GetArrayItem` _cards (`KismetArrayLibrary.Array_LastIndex` _cards))))