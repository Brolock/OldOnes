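; BP_Relic is a relic component that fires abilities on pickup, use or removal, as its flags allow.
; It adds an ability manager to its owner, requests targets when triggered, and executes the abilities through a target-ready callback.
; Usable relics count down uses and attempt removal at zero, with destruction deferred in Tick while targets are pending.
; It can pack its settings and abilities into a relic data struct.
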(event `self.ReceiveBeginPlay`
  (bind _returnvalue (`|AddComponentByClass` (`self.GetOwner`) "/Game/OldOnes/Core/Abilities/BP_AbilityManager.BP_AbilityManager_C"))
  (bind _output_get (set `self.RelicAbilities` _returnvalue))
  (add `/Game/OldOnes/Core/Abilities/BP_AbilityManager.TargetsReadyForExecution` _output_get (`|CreateDelegate` :!event `ExecuteAbilities`))
  (if (> (`KismetArrayLibrary.Array_Length` (`self.Abilities`)) 0)
    (`/Game/OldOnes/Core/Abilities/BP_AbilityManager.AddAbilities` (`self.RelicAbilities`) (`self.Abilities`))))

(event `self.ReceiveTick`
  (params (DeltaSeconds :type "Float (single-precision)"))
  (if (and (`self.QueuedForDestruction`) (not (`self.WaitingForTargets`)))
    (`self.RemoveRelicEvent` self)
    (`self.K2_DestroyComponent`)))

(fn `DestroyRelic`
  (set `self.QueuedForDestruction` true))

(fn `ExecuteAbilities`
  (params (FiringAbilityManager :type "/Game/OldOnes/Core/Abilities/BP_AbilityManager Object Reference"))
  (`/Game/OldOnes/Core/Abilities/BP_AbilityManager.ExecuteAbilities` FiringAbilityManager)
  (set `self.WaitingForTargets` false)
  (if (and (`self.IsUsable`) (== (`self.NumberOfUses`) 0))
    (`self.RemoveRelic`)))

(fn `PackRelicToStruct`
  (returns (RelicStruct :type "/Game/OldOnes/Core/Relics/SRelicData Structure"))
  (return (make `/Game/OldOnes/Core/Relics/SRelicData` (`GameplayStatics.GetObjectClass` self) (`self.Name`) (`self.ShownText`) "NewEnumerator0" (`self.IsRemovable`) (`self.IsUsable`) (`self.NumberOfUses`) (`/Game/OldOnes/Core/Abilities/BP_AbilityManager.PackAbilitiesToStruct` (`self.RelicAbilities`)) (`self.AbilitiesTriggerOnPickup`) (`self.AbilitiesTriggerOnRemoval`) (`self.AbilitiesTriggerOnUse`) (`self.RelicIcon`) (`self.StacksIcon`))))

(fn `Relic Picked`
  (if (`self.AbilitiesTriggerOnPickup`)
    (`self.TriggerRelic`)))

(fn `RelicRemovedTrigger`
  (if (`self.AbilitiesTriggerOnRemoval`)
    (`self.TriggerRelic`)))

(fn `RemoveRelic`
  (if (`self.IsRemovable`)
    (`self.RelicRemovedTrigger`)
    (`self.DestroyRelic`)
    (else
      (`/Game/OldOnes/Core/Tools/BPFL_WidgetUtilities.Display Message to User` (`|FormatText` "{RelicName} cannot be removed!" (`self.Name`))))))

(fn `TriggerRelic`
  (set `self.WaitingForTargets` true)
  (`self.RelicTriggersEvent`)
  (`/Game/OldOnes/Core/Abilities/BP_AbilityManager.GetTargets` (`self.RelicAbilities`)))

(fn `UseRelic`
  (if (`self.IsUsable`)
    (if (`self.AbilitiesTriggerOnUse`)
      (`/Engine/EditorBlueprintResources/StandardMacros.DecrementInt` (`self.NumberOfUses`)
        (:`  `
          (`self.TriggerRelic`))))
    (else
      (`KismetSystemLibrary.PrintString` "BP_Relic::UseRelic: Trying to Use a relic that is not usable." true true (struct :`R` 1.0 :`B` 0.03269 :`A` 1.0) 30.0))))