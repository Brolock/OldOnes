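; BP_RelicManager holds the player's relics up to a capacity limit and packs them into structs.
; AddRelic picks up relics while space remains, binding their removal event to drop them from the list.
; Tick picks up any queued relic once space frees.
; When full, AddRelic shows a message if all relics are locked, but both full branches act on RelicQueuedForAdd, so NewRelic is never queued or destroyed.
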(event `self.ReceiveTick`
  (params (DeltaSeconds :type "Float (single-precision)"))
  (if (and (`KismetSystemLibrary.IsValid` (`self.RelicQueuedForAdd`)) (not (`self.IsFull`)))
    (`self.PickupRelic` (`self.RelicQueuedForAdd`))
    (set `self.RelicQueuedForAdd` null)))

(fn `AddRelic`
  (params (NewRelic :type "/Game/OldOnes/Core/Relics/BP_Relic Object Reference"))
  (if (`self.IsFull`)
    (if (`self.Are All Relics Locked`)
      (`/Game/OldOnes/Core/Tools/BPFL_WidgetUtilities.Display Message to User` "All relics are locked, you cannot add a new one.")
      (`/Game/OldOnes/Core/Relics/BP_Relic.DestroyRelic` (`self.RelicQueuedForAdd`))
      (else
        (`/Engine/EditorBlueprintResources/StandardMacros.IsValid` (`self.RelicQueuedForAdd`)
          (:`Is Valid`
            (`KismetSystemLibrary.PrintString` "BP_RelicManager::AddRelic: Trying to add a relic while another one is already queued. Some logic needs to be changed " true true (struct :`R` 1.0 :`B` 0.005552 :`A` 1.0) 30.0))
          (:`Is Not Valid`
            (set `self.RelicQueuedForAdd` (`self.RelicQueuedForAdd`))))))
    (else
      (`self.PickupRelic` (`local.NewRelic`)))))

(fn `Are All Relics Locked`
  (returns (AllLocked :type Boolean))
  (for _array_element (`self.Relics`)
    (if (`/Game/OldOnes/Core/Relics/BP_Relic.IsRemovable` _array_element)
      (return false)))
  (return true))

(fn `IsFull`
  (returns (IsFull :type Boolean))
  (return (== (`KismetArrayLibrary.Array_Length` (`self.Relics`)) (`self.MaxRelics`))))

(fn `PackToStruct`
  (returns (RelicsPacked :type "Array of /Game/OldOnes/Core/Relics/SRelicData Structure"))
  (locals (LocalRelicsPacked :type "Array of /Game/OldOnes/Core/Relics/SRelicData Structure"))
  (for _array_element (`self.Relics`)
    (bind _relicstruct (`/Game/OldOnes/Core/Relics/BP_Relic.PackRelicToStruct` _array_element))
    (`KismetArrayLibrary.Array_Add` (`local.LocalRelicsPacked`) _relicstruct))
  (return (`local.LocalRelicsPacked`)))

(fn `PickupRelic`
  (params (NewRelic :type "/Game/OldOnes/Core/Relics/BP_Relic Object Reference"))
  (add `/Game/OldOnes/Core/Relics/BP_Relic.RemoveRelicEvent` NewRelic (`|CreateDelegate` :!event `RemoveRelicForward`))
  (`KismetArrayLibrary.Array_Add` (`self.Relics`) NewRelic)
  (`/Game/OldOnes/Core/Relics/BP_Relic.Relic Picked` NewRelic))

(fn `RemoveRelicForward`
  (params (CallingRelic :type "/Game/OldOnes/Core/Relics/BP_Relic Object Reference"))
  (bind _returnvalue (`KismetArrayLibrary.Array_RemoveItem` (`self.Relics`) CallingRelic))
  (if (not _returnvalue)
    (`KismetSystemLibrary.PrintString` "BP_RelicManager::RemoveRelic: Remove not in container was called for removal. Look into it" true true (struct :`R` 1.0 :`B` 0.028497 :`A` 1.0) 30.0)))