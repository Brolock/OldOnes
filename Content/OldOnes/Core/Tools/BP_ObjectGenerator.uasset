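; Generator that creates cards and relics from data tables for rewards and in-game effects, resolving queued queries one at a time, cards before relics.
; Cards come by name or type; random picks roll rarities from the seeded game stream, then scan shuffled rows, lowering rarity when matches run out.
; Results go to a multi-option pick screen or straight to the run deck, fight piles (full hand redirects) or relic manager.
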(event `self.ReceiveBeginPlay`)

(fn `Card Created Selected`
  (params (CardView :type "/Game/OldOnes/Core/PlayerUI/WBP_CardView Object Reference"))
  (bind (_carddatatable _cardnames _cardtypesfilter _numberofcardstogenerate _cardraritydroppecent _arecreatedcardstobepicked _addcardstorundeck _fightmodecardsdestination) (break `/Game/OldOnes/Core/Tools/SCardGenerationQuery` (`|GetArrayItem` (`self.CardGenerationQueries`))))
  (`self.FinalizeCardCreation` (`|MakeArray` CardView) _addcardstorundeck _fightmodecardsdestination))

(fn `FinalizeCardCreation`
  (params (CardsCreated :type "Array of /Game/OldOnes/Core/PlayerUI/WBP_CardView Object Reference") (AddCardToRunDeck :type Boolean) (CardDestination :type "/Game/OldOnes/Core/Cards/ECardLocation Enum" :default "NewEnumerator5"))
  (locals (CardLocation :type "/Game/OldOnes/Core/Cards/ECardLocation Enum" :default "NewEnumerator5") (ViewToAdd :type "/Game/OldOnes/Core/PlayerUI/WBP_CardView Object Reference") (CardToAdd :type "/Game/OldOnes/Core/Cards/BP_Card Object Reference") (AddCardToPile :type Boolean))
  (bind _cardtoadd (`local.CardToAdd`))
  (bind (_cardpile _collectionview) (`/Game/OldOnes/Core/Tools/BPFL_GeneralFunctions.Convert Location Enum to Component Ref` (`local.CardLocation`)))
  (if (and (`|EnumInequality` CardDestination "NewEnumerator5") (`/Game/OldOnes/Core/Tools/BPFL_GeneralFunctions.IsEncounterTypeFight`))
    (set `local.CardLocation` CardDestination)
    (set `local.AddCardToPile` true))
  (for _array_element (`local.CardsCreated`)
    (bind _output_get (set `local.ViewToAdd` _array_element))
    (set `local.CardToAdd` (`/Game/OldOnes/Core/PlayerUI/WBP_CardView.ViewedCard` _output_get))
    (if (`local.AddCardToRunDeck`)
      ;[0.3558 1 0.4534] Add card to run deck
      (`/Game/OldOnes/Core/Tools/BPFL_Cards.AddCardToRunDeck` _cardtoadd)
      (`self.Move Card View to Container` (`local.ViewToAdd`) (`/Game/OldOnes/Core/GameUI/WBP_GameUI.RunDeckView` (`/Game/OldOnes/Core/Tools/BPFL_GeneralFunctions.GetGameUI`)))
      ;[1 0.9782 0] Make a copy of the card to add to the fight deck
      (if (`local.AddCardToPile`)
        (bind (_card _view) (`/Game/OldOnes/Core/Tools/BPFL_Cards.CreateCardAndViewFromStruct` (`/Game/OldOnes/Core/Cards/BP_Card.PackCardToStruct` _cardtoadd) (`/Game/OldOnes/Core/Tools/BPFL_GeneralFunctions.GetCardPlayerPawn`)))
        (set `local.CardToAdd` _card)
        (set `local.ViewToAdd` _view)
        ;[1 0.5997 0.04934] Add card to pile in combat
        (bind _asbp_hand_manager (cast `/Game/OldOnes/Core/CardPile/BP_HandManager` _cardpile :!label _label)
          (:`then`
            (if (`/Game/OldOnes/Core/CardPile/BP_HandManager.IsHandFull` _asbp_hand_manager)
              (bind _output_get_2 (set `local.CardLocation` "NewEnumerator1"))
              (bind (_cardpile_2 _collectionview_2) (`/Game/OldOnes/Core/Tools/BPFL_GeneralFunctions.Convert Location Enum to Component Ref` _output_get_2))
              (bind _asbp_card_pile (cast `/Game/OldOnes/Core/CardPile/BP_CardPile` _cardpile_2))
              (`/Game/OldOnes/Core/CardPile/BP_CardPile.AddCardToPile` _asbp_card_pile (`local.CardToAdd`) "NewEnumerator0" false)
              (`self.Move Card View to Container` (`local.ViewToAdd`) _collectionview_2)
              (else
                (`/Game/OldOnes/Core/CardPile/BP_HandManager.AddCardToHand` _asbp_hand_manager (`local.CardToAdd`))
                (`self.Move Card View to Container` (`local.ViewToAdd`) _collectionview :!label _label_2))))
          (:`CastFailed`
            (bind _asbp_card_pile_2 (cast `/Game/OldOnes/Core/CardPile/BP_CardPile` _cardpile))
            (`/Game/OldOnes/Core/CardPile/BP_CardPile.AddCardToPile` _asbp_card_pile_2 (`local.CardToAdd`) "NewEnumerator0" (`|EnumEquality` (`local.CardLocation`) "NewEnumerator0"))
            (goto _label_2))))
      (else
        (goto _label))))
  (`KismetArrayLibrary.Array_Remove` (`self.CardGenerationQueries`))
  (set `self.ResolvingGeneration` false)
  (`self.GoToNextGenerationQuery`))

(fn `FinalizeRelicCreation`
  (params (RelicViews :type "Array of /Game/OldOnes/Core/Relics/WBP_RelicView Object Reference"))
  (for _array_element RelicViews
    (`/Game/OldOnes/Core/Relics/BP_RelicManager.AddRelic` (`/Game/OldOnes/Core/Tools/BPFL_Relics.GetRelicsManager`) (`/Game/OldOnes/Core/Relics/WBP_RelicView.ViewedRelic` _array_element))
    (`/Game/OldOnes/Core/Relics/WBP_RelicManagerView.AddRelicView` (`/Game/OldOnes/Core/GameUI/WBP_GameUI.RelicManagerView` (`/Game/OldOnes/Core/Tools/BPFL_GeneralFunctions.GetGameUI`)) _array_element))
  (`KismetArrayLibrary.Array_Remove` (`self.RelicGenerationQueries`))
  (set `self.ResolvingGeneration` false)
  (`self.GoToNextGenerationQuery`))

(fn `GenerateCardsByName`
  (params (CardName :type "Array of Name") (DataTable :type "DataTable Object Reference"))
  (returns (CreatedCardsViews :type "Array of /Game/OldOnes/Core/PlayerUI/WBP_CardView Object Reference"))
  (locals (LocalCreatedCardsViews :type "Array of /Game/OldOnes/Core/PlayerUI/WBP_CardView Object Reference"))
  (for _array_element CardName
    ;[1 0.2321 0] Card Owner is game mode, maybe not the best
    (bind (_card _view) (`/Game/OldOnes/Core/Tools/BPFL_Cards.CreateCardAndViewFromName` _array_element (`/Game/OldOnes/Core/Tools/BPFL_GeneralFunctions.GetCardGameMode`) DataTable))
    (`KismetArrayLibrary.Array_Add` (`local.LocalCreatedCardsViews`) _view))
  (return (`local.LocalCreatedCardsViews`)))

(fn `GenerateCardsByType`
  (params (CardTypeFilter :type "Set of /Game/OldOnes/Core/Cards/ECardTypes Enum") (NumberOfCards :type Integer) (DataTable :type "DataTable Object Reference"))
  (returns (GeneratedCardViews :type "Array of /Game/OldOnes/Core/PlayerUI/WBP_CardView Object Reference"))
  (locals (GeneratedViews :type "Array of /Game/OldOnes/Core/PlayerUI/WBP_CardView Object Reference"))
  (bind _rarityofobjects (`self.Random Sample Of Rarities` NumberOfCards (`self.RarityPercentage`)))
  (bind _cardspicked (`self.MakeCardStructsFromRarityAndType` CardTypeFilter _rarityofobjects DataTable))
  (for _array_element _cardspicked
    ;[1 0.1687 0] Card's owner is the game mode as default, not sure this is the best decision
    (bind (_card _view) (`/Game/OldOnes/Core/Tools/BPFL_Cards.CreateCardAndViewFromStruct` _array_element (`/Game/OldOnes/Core/Tools/BPFL_GeneralFunctions.GetCardGameMode`)))
    (`KismetArrayLibrary.Array_Add` (`local.GeneratedViews`) _view))
  (return (`local.GeneratedViews`)))

(fn `GenerateRelics`
  (params (RelicDataTable :type "DataTable Object Reference") (NumberOfRelics :type Integer))
  (returns (RelicViews :type "Array of /Game/OldOnes/Core/Relics/WBP_RelicView Object Reference"))
  (locals (RelicViewsGenerated :type "Array of /Game/OldOnes/Core/Relics/WBP_RelicView Object Reference"))
  (bind _rarityofobjects (`self.Random Sample Of Rarities` NumberOfRelics (`self.RarityPercentage`)))
  (bind _relicstructs (`self.MakeRelicStructsFromRarity` _rarityofobjects RelicDataTable))
  (for _array_element _relicstructs
    (bind (_relic _relicview) (`/Game/OldOnes/Core/Tools/BPFL_Relics.CreateRelicAndViewFromStuct` _array_element))
    (`KismetArrayLibrary.Array_Add` (`local.RelicViewsGenerated`) _relicview))
  (return (`local.RelicViewsGenerated`)))

(fn `GoToNextGenerationQuery`
  (if (not (`self.ResolvingGeneration`))
    (if (> (`KismetArrayLibrary.Array_Length` (`self.CardGenerationQueries`)) 0)
      (`self.ResolveCardGenerationQuery` (`|GetArrayItem` (`self.CardGenerationQueries`)))
      (elif (> (`KismetArrayLibrary.Array_Length` (`self.RelicGenerationQueries`)) 0)
        (`self.ResolveRelicGenerationQuery` (`|GetArrayItem` (`self.RelicGenerationQueries`)))
        (else
          (`self.QueriesCleared`))))))

(fn `Lower Rarity Array`
  (params (Rarities :type "Array of /Game/OldOnes/Core/Cards/ERarity Enum (by ref)"))
  (for (_array_element _array_index) Rarities
    (switch `/Game/OldOnes/Core/Cards/ERarity` _array_element
      (:`NewEnumerator0`
        (`KismetArrayLibrary.Array_Set` (`local.Rarities`) _array_index "NewEnumerator0")
        (`KismetSystemLibrary.PrintString` "BP_CardGenerator::LowerRarityArray: Trying to lower rarity of a common card. This means there is not enough cards for your generation. Probably looping infinitely" true true (struct :`R` 1.0 :`A` 1.0) 30.0))
      (:`NewEnumerator1`
        (`KismetArrayLibrary.Array_Set` (`local.Rarities`) _array_index "NewEnumerator0"))
      (:`NewEnumerator2`
        (`KismetArrayLibrary.Array_Set` (`local.Rarities`) _array_index "NewEnumerator1"))
      (:`NewEnumerator3`
        (`KismetArrayLibrary.Array_Set` (`local.Rarities`) _array_index "NewEnumerator3")
        (`KismetSystemLibrary.PrintString` "BP_CardGenerator::LowerRarityArray: Trying to lower rarity of a base card. This means there is not enough cards for your generation. Probably looping infinitely" true true (struct :`R` 1.0 :`A` 1.0) 30.0)))))

(fn `MakeCardStructsFromRarityAndType`
  (params (CardsTypes :type "Set of /Game/OldOnes/Core/Cards/ECardTypes Enum") (CardsRarity :type "Array of /Game/OldOnes/Core/Cards/ERarity Enum") (DataTable :type "DataTable Object Reference"))
  (returns (CardsPicked :type "Array of /Game/OldOnes/Core/Cards/SCardData Structure"))
  (locals (CardsPickedLocal :type "Array of /Game/OldOnes/Core/Cards/SCardData Structure"))
  (bind _cardsrarity (`local.CardsRarity`))
  (bind _cardspickedlocal (`local.CardsPickedLocal`))
  (bind _outrownames (`DataTableFunctionLibrary.GetDataTableRowNames` DataTable))
  (`KismetArrayLibrary.Array_Shuffle` _outrownames)
  (while (> (`KismetArrayLibrary.Array_Length` (`local.CardsRarity`)) 0)
    ;[1 1 1] Find Cards of required rarity
    (for _array_element _outrownames
      (bind _returnvalue (`|GetDataTableRow` (`local.DataTable`) _array_element)
        (:`then`
          (bind (_name _manacost _cardtype _cardclass _madnesslevel _rarity) (break `/Game/OldOnes/Core/Cards/SCardData` _returnvalue))
          (bind _returnvalue_2 (`KismetArrayLibrary.Array_Find` (`local.CardsRarity`) _rarity))
          (if (and (not (`KismetArrayLibrary.Array_Contains` _cardspickedlocal _returnvalue)) (`BlueprintSetLibrary.Set_Contains` (`local.CardsTypes`) _cardtype) (!= _returnvalue_2 -1))
            (`KismetArrayLibrary.Array_Add` _cardspickedlocal _returnvalue)
            (`KismetArrayLibrary.Array_Remove` _cardsrarity _returnvalue_2)
            (if (== (`KismetArrayLibrary.Array_Length` _cardsrarity) 0)
              (break))))))
    (`self.Lower Rarity Array` (`local.CardsRarity`)))
  (return (`local.CardsPickedLocal`)))

(fn `MakeRelicStructsFromRarity`
  (params (RelicsRarities :type "Array of /Game/OldOnes/Core/Cards/ERarity Enum") (DataTable :type "DataTable Object Reference"))
  (returns (RelicStructs :type "Array of /Game/OldOnes/Core/Relics/SRelicData Structure"))
  (locals (RelicStructsLocal :type "Array of /Game/OldOnes/Core/Relics/SRelicData Structure"))
  (bind _relicstructslocal (`local.RelicStructsLocal`))
  (bind _relicsrarities (`local.RelicsRarities`))
  (bind _outrownames (`DataTableFunctionLibrary.GetDataTableRowNames` DataTable))
  (`KismetArrayLibrary.Array_Shuffle` _outrownames)
  (while (> (`KismetArrayLibrary.Array_Length` (`local.RelicsRarities`)) 0)
    ;[1 1 1] Pick relics of the desired rarity (or lower if not enough relics of the desired rarity exist)
    (for _array_element _outrownames
      (bind _returnvalue (`|GetDataTableRow` (`local.DataTable`) _array_element)
        (:`then`
          (bind _returnvalue_2 (`KismetArrayLibrary.Array_Find` (`local.RelicsRarities`) (`.RelicRarity_38_01E4260645999BE33EFE74AAA11D3F01` (break `/Game/OldOnes/Core/Relics/SRelicData` _returnvalue))))
          (if (and (not (`KismetArrayLibrary.Array_Contains` _relicstructslocal _returnvalue)) (!= _returnvalue_2 -1))
            (`KismetArrayLibrary.Array_Add` _relicstructslocal _returnvalue)
            (`KismetArrayLibrary.Array_Remove` _relicsrarities _returnvalue_2)
            (if (== (`KismetArrayLibrary.Array_Length` _relicsrarities) 0)
              (break))))))
    (`self.Lower Rarity Array` (`local.RelicsRarities`)) ; Lower Rarities to find leftover items
  )
  (return (`local.RelicStructsLocal`)))

(fn `Move Card View to Container`
  (params (CardView :type "/Game/OldOnes/Core/PlayerUI/WBP_CardView Object Reference") (Container :type "/Game/OldOnes/Core/PlayerUI/WBP_CardContainerParent Object Reference"))
  (bind _temporarycanvas (`/Game/OldOnes/Core/GameUI/WBP_MultiOptionsScreen.TemporaryCanvas` (`/Game/OldOnes/Core/GameUI/WBP_GameUI.MultiOptionsPopUp` (`/Game/OldOnes/Core/Tools/BPFL_GeneralFunctions.GetGameUI`))))
  (`CanvasPanel.AddChildToCanvas` _temporarycanvas CardView)
  (`/Game/OldOnes/Core/PlayerUI/WBP_CardContainerParent.AddCardToContainer` Container CardView _temporarycanvas))

(fn `QueryForCards`
  (params (CardQuery :type "/Game/OldOnes/Core/Tools/SCardGenerationQuery Structure"))
  (`KismetArrayLibrary.Array_Add` (`self.CardGenerationQueries`) CardQuery)
  (`self.GoToNextGenerationQuery`))

(fn `QueryForRelics`
  (params (RelicQuery :type "/Game/OldOnes/Core/Tools/SRelicGenerationQuery Structure"))
  (`KismetArrayLibrary.Array_Add` (`self.RelicGenerationQueries`) RelicQuery)
  (`self.GoToNextGenerationQuery`))

(fn `Random Sample Of Rarities`
  (params (NumberOfObjects :type Integer) (RarityDropPercent :type "Map of /Game/OldOnes/Core/Cards/ERarity Enum to Float (double-precision)"))
  (returns (RarityOfObjects :type "Array of /Game/OldOnes/Core/Cards/ERarity Enum"))
  (locals (RareThreshold :type "Float (double-precision)") (UncommonThreshold :type "Float (double-precision)") (RandomPick :type "Float (double-precision)") (RarityOfCardsLocal :type "Array of /Game/OldOnes/Core/Cards/ERarity Enum"))
  (bind _rarityofcardslocal (`local.RarityOfCardsLocal`))
  (bind _output_get (set `local.RareThreshold` (`BlueprintMapLibrary.Map_Find` RarityDropPercent "NewEnumerator2")))
  (set `local.UncommonThreshold` (+ _output_get (`BlueprintMapLibrary.Map_Find` RarityDropPercent "NewEnumerator1")))
  (for _ (range (`local.NumberOfObjects`))
    (bind _output_get_2 (set `local.RandomPick` (* (`KismetMathLibrary.RandomFloatFromStream` (`/Game/OldOnes/Core/Tools/BPFL_GeneralFunctions.GetGameRandomStream`)) 100.0)))
    (if (< _output_get_2 (`local.RareThreshold`))
      (`KismetArrayLibrary.Array_Add` _rarityofcardslocal "NewEnumerator2")
      (elif (< _output_get_2 (`local.UncommonThreshold`))
        (`KismetArrayLibrary.Array_Add` _rarityofcardslocal "NewEnumerator1")
        (else
          (`KismetArrayLibrary.Array_Add` _rarityofcardslocal "NewEnumerator0")))))
  (return (`local.RarityOfCardsLocal`)))

(fn `RelicCreatedSelected`
  (params (RelicView :type "/Game/OldOnes/Core/Relics/WBP_RelicView Object Reference"))
  (`self.FinalizeRelicCreation` (`|MakeArray` RelicView)))

(fn `ResolveCardGenerationQuery`
  (params (CardGenQuery :type "/Game/OldOnes/Core/Tools/SCardGenerationQuery Structure"))
  (locals (ViewsGenerated :type "Array of /Game/OldOnes/Core/PlayerUI/WBP_CardView Object Reference") (CardDataTable :type "DataTable Object Reference"))
  (bind (_carddatatable _cardnames _cardtypesfilter _numberofcardstogenerate _cardraritydroppecent) (break `/Game/OldOnes/Core/Tools/SCardGenerationQuery` CardGenQuery))
  (bind _multioptionsscreen (`/Game/OldOnes/Core/Tools/BPFL_WidgetUtilities.GetMultiOptionsScreen`))
  (bind (_carddatatable_2 _cardnames_2 _cardtypesfilter_2 _numberofcardstogenerate_2 _cardraritydroppecent_2 _arecreatedcardstobepicked _addcardstorundeck _fightmodecardsdestination) (break `/Game/OldOnes/Core/Tools/SCardGenerationQuery` (`local.CardGenQuery`)))
  (set `self.ResolvingGeneration` true)
  (set `local.CardDataTable` _carddatatable)
  (if (!= (`KismetArrayLibrary.Array_Length` _cardnames) 0)
    (bind _createdcardsviews (`self.GenerateCardsByName` _cardnames (`local.CardDataTable`)))
    (set `local.ViewsGenerated` _createdcardsviews)
    (else
      (set `self.RarityPercentage` _cardraritydroppecent)
      (bind _generatedcardviews (`self.GenerateCardsByType` _cardtypesfilter _numberofcardstogenerate (`local.CardDataTable`)))
      (set `local.ViewsGenerated` _generatedcardviews)))
  (if _arecreatedcardstobepicked
    (add `/Game/OldOnes/Core/GameUI/WBP_MultiOptionsScreen.CardSelectedEvent` _multioptionsscreen (`|CreateDelegate` :!event `Card Created Selected`))
    (`/Game/OldOnes/Core/GameUI/WBP_MultiOptionsScreen.AddCards` _multioptionsscreen (`local.ViewsGenerated`))
    (else
      (`self.FinalizeCardCreation` (`local.ViewsGenerated`) _addcardstorundeck _fightmodecardsdestination))))

(fn `ResolveRelicGenerationQuery`
  (params (RelicGenQuery :type "/Game/OldOnes/Core/Tools/SRelicGenerationQuery Structure"))
  (bind (_relicdatatable _relicraritydroppercent _numberofrelicstogenerate _arerelicstobepicked) (break `/Game/OldOnes/Core/Tools/SRelicGenerationQuery` RelicGenQuery))
  (bind _multioptionsscreen (`/Game/OldOnes/Core/Tools/BPFL_WidgetUtilities.GetMultiOptionsScreen`))
  (set `self.ResolvingGeneration` true)
  (set `self.RarityPercentage` _relicraritydroppercent)
  (bind _relicviews (`self.GenerateRelics` _relicdatatable _numberofrelicstogenerate))
  (if _arerelicstobepicked
    (add `/Game/OldOnes/Core/GameUI/WBP_MultiOptionsScreen.RelicSelectedEvent` _multioptionsscreen (`|CreateDelegate` :!event `RelicCreatedSelected`))
    (`/Game/OldOnes/Core/GameUI/WBP_MultiOptionsScreen.AddRelics` _multioptionsscreen _relicviews)
    (else
      (`self.FinalizeRelicCreation` _relicviews))))