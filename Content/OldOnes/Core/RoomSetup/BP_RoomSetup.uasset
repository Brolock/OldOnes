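; Room layout actor that gathers enemy and boss spawn location components placed in it and reports how many slots of each it offers.
; Construction script sorts child location components into enemy and boss lists.
; In non-packaged builds it previews them with placeholder animated meshes and colored index labels, plus a room index from its position among all room setups, using a random color if unset.
; Hidden, without collision at runtime.
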(event `self.ReceiveBeginPlay`
  (`self.SetActorHiddenInGame` true)
  (`self.SetActorEnableCollision` false))

(fn `CurrentRoomIdxVisualText`
  (params (RoomIdx :type Integer) (TextColor :type "Color Structure"))
  (if (not (`self.DisableEnemiesAndRoomIndexText`))
    (bind _returnvalue (`|AddComponentByClass` "/Script/Engine.TextRenderComponent" false (`KismetMathLibrary.MakeTransform` (0.0 0.0 0.0) (struct) (6.0 6.0 6.0))))
    (`TextRenderComponent.SetHorizontalAlignment` _returnvalue "EHTA_Center")
    (`TextRenderComponent.K2_SetText` _returnvalue (`KismetTextLibrary.Conv_IntToText` RoomIdx))
    (`TextRenderComponent.SetTextRenderColor` _returnvalue TextColor)))

(fn `GetAvailableSlots`
  (returns (NumberOfEnemiesSlots :type Integer) (NumberOfBossSlots :type Integer))
  (return (`KismetArrayLibrary.Array_Length` (`self.RoomEnemiesLocations`)) (`KismetArrayLibrary.Array_Length` (`self.RoomBossesLocations`))))

(fn `SetupEnemyLocationVisual`
  (params (EnemyLocation :type "/Game/OldOnes/Core/RoomSetup/BP_EnemyRoomLocation Object Reference") (EnemyIdxInRoom :type Integer) (IdxTextSize :type "Float (double-precision)"))
  (locals (SkeletalMesh :type "SkeletalMeshComponent Object Reference") (LocationText :type "TextRenderComponent Object Reference"))
  (bind _enemylocation (`local.EnemyLocation`))
  (bind _locationtext (`local.LocationText`))
  (bind _relativescale3d (`SceneComponent.RelativeScale3D` (`local.EnemyLocation`)))
  (if (`self.EnableSkeletalMeshes`)
    ;[0.439 1 0.4515] Set the default SkeletalMesh and animation to be displayed
    (bind _returnvalue (`|AddComponentByClass` "/Script/Engine.SkeletalMeshComponent"))
    (bind _output_get (set `local.SkeletalMesh` _returnvalue))
    (bind _returnvalue_2 (`KismetSystemLibrary.LoadAsset_Blocking` (`/Game/OldOnes/Core/RoomSetup/BP_EnemyRoomLocation.PlaceHolderSkeletalMesh` _enemylocation)))
    (bind _asskeletal_mesh (cast `SkeletalMesh` _returnvalue_2))
    (`SkinnedMeshComponent.SetSkinnedAssetAndUpdate` _output_get _asskeletal_mesh true)
    (bind _returnvalue_3 (`KismetSystemLibrary.LoadAsset_Blocking` (`/Game/OldOnes/Core/RoomSetup/BP_EnemyRoomLocation.PlaceholderAnimation` _enemylocation)))
    (bind _asanim_sequence (cast `AnimSequence` _returnvalue_3))
    (`SkeletalMeshComponent.OverrideAnimationData` _output_get _asanim_sequence true true 0.0 1.0)
    (`SceneComponent.K2_AttachToComponent` _output_get (`local.EnemyLocation`) "None" "KeepRelative" "KeepRelative" "KeepRelative" true)
    ;[0.3468 0.1768 0.6458] Make the text centered on top of the SkeletalMesh
    (if (not (`self.DisableEnemiesAndRoomIndexText`))
      (bind _returnvalue_4 (`|AddComponentByClass` "/Script/Engine.TextRenderComponent" false (`KismetMathLibrary.MakeTransform` (/ (`KismetMathLibrary.MakeVector` 0.0 0.0 (* (.z (`.BoxExtent` (`KismetSystemLibrary.GetComponentBounds` (`local.SkeletalMesh`)))) 2.0)) _relativescale3d) (struct) (* (/ (1.0 1.0 1.0) _relativescale3d) (`local.IdxTextSize`)))))
      (set `local.LocationText` _returnvalue_4)
      (`TextRenderComponent.SetHorizontalAlignment` (`local.LocationText`) "EHTA_Center" :!label _label)
      ;[1 1 1] Each enemy location has its ID printed on top of it
      (`TextRenderComponent.K2_SetText` _locationtext (`KismetTextLibrary.Conv_IntToText` (`local.EnemyIdxInRoom`)))
      (`TextRenderComponent.SetTextRenderColor` _locationtext (`self.RoomColor`))
      (`SceneComponent.K2_AttachToComponent` _locationtext (`local.EnemyLocation`) "None" "KeepRelative" "KeepWorld" "KeepRelative" true))
    (elif (not (`self.DisableEnemiesAndRoomIndexText`))
      (bind _returnvalue_5 (`|AddComponentByClass` "/Script/Engine.TextRenderComponent" false (`KismetMathLibrary.MakeTransform` (0.0 0.0 0.0) (struct) (* (/ (1.0 1.0 1.0) (`SceneComponent.RelativeScale3D` (`local.EnemyLocation`))) (`local.IdxTextSize`)))))
      (set `local.LocationText` _returnvalue_5)
      (goto _label))))

(fn `SetupRoomVisualization`
  (if (== (`.A` (break `Color` (`self.RoomColor`))) 0)
    (set `self.RoomColor` (`KismetMathLibrary.Conv_LinearColorToColor` (`KismetMathLibrary.MakeColor` (`KismetMathLibrary.RandomFloatInRange` 0.0 1.0) (`KismetMathLibrary.RandomFloatInRange` 0.0 1.0) (`KismetMathLibrary.RandomFloatInRange` 0.0 1.0)))))
  (bind _outactors (`GameplayStatics.GetAllActorsOfClass` "BP_RoomSetup_C"))
  (`self.CurrentRoomIdxVisualText` (`KismetArrayLibrary.Array_Find` _outactors self) (`self.RoomColor`))
  (for (_array_element _array_index) (`self.RoomEnemiesLocations`)
    (`self.SetupEnemyLocationVisual` _array_element _array_index (`self.EnemyIdxTextSize`)))
  (for (_array_element_2 _array_index_2) (`self.RoomBossesLocations`)
    (`self.SetupEnemyLocationVisual` _array_element_2 _array_index_2 (`self.BossIdxTextSize`))))

(fn `UserConstructionScript`
  (for _array_element (`self.K2_GetComponentsByClass` "/Game/OldOnes/Core/RoomSetup/BP_EnemyRoomLocation.BP_EnemyRoomLocation_C")
    (bind _asbp_boss_room_location (cast `/Game/OldOnes/Core/RoomSetup/BP_BossRoomLocation` _array_element)
      (:`then`
        (`KismetArrayLibrary.Array_Add` (`self.RoomBossesLocations`) _asbp_boss_room_location))
      (:`CastFailed`
        (`KismetArrayLibrary.Array_Add` (`self.RoomEnemiesLocations`) _array_element))))
  (if (not (`KismetSystemLibrary.IsPackagedForDistribution`))
    (`self.SetupRoomVisualization`)))