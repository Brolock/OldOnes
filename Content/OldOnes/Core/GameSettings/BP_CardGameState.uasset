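; Game state for the card game that starts a run's combat setup and hosts shared manager objects.
; On BeginPlay it reads the run info from the card game instance and initializes the player pawn's stats and deck.
; Construction creates a widget movement manager and an ability targeting manager, exposed through getters.
; Tick drives the movement manager to animate widgets each frame.
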(event `self.ReceiveBeginPlay`
  (bind (_rundeck _playerstats) (`/Game/OldOnes/Core/GameSettings/BP_CardGameInstance.Get Run Infos` (`/Game/OldOnes/Core/Tools/BPFL_GeneralFunctions.GetCardGameInstance`)))
  (`/Game/OldOnes/Core/Player/BP_PlayerPawn.Initialize Player From State Struct` (`/Game/OldOnes/Core/Tools/BPFL_GeneralFunctions.GetCardPlayerPawn`) _playerstats)
  (`/Game/OldOnes/Core/Player/BP_PlayerPawn.InitializeDeck` (`/Game/OldOnes/Core/Tools/BPFL_GeneralFunctions.GetCardPlayerPawn`) _rundeck))

(event `self.ReceiveTick`
  (params (DeltaSeconds :type "Float (single-precision)"))
  (`/Game/OldOnes/Core/UI/BP_WidgetMovementManager.MoveWidgets` (`self.WidgetMovementManager`) DeltaSeconds))

(fn `GetAbilityTargetingManager`
  (returns (AbilityTargetingManager :type "/Game/OldOnes/Core/Abilities/BP_AbilityTargetingManager Object Reference"))
  (return (`self.AbilityTargetingManager`)))

(fn `GetWidgetMovementManager`
  (returns (WidgetMovementManager :type "/Game/OldOnes/Core/UI/BP_WidgetMovementManager Object Reference"))
  (return (`self.WidgetMovementManager`)))

(fn `UserConstructionScript`
  (bind _returnvalue (`|GenericCreateObject` "/Game/OldOnes/Core/UI/BP_WidgetMovementManager.BP_WidgetMovementManager_C" self))
  (set `self.WidgetMovementManager` _returnvalue)
  (bind _returnvalue_2 (`AddComponent|NODE_AddBP_AbilityTargetingManager-0`))
  (set `self.AbilityTargetingManager` _returnvalue_2))