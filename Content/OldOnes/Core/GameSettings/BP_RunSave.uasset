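; BP_RunSave holds the saved state of a run in a card-based game with a world map, bioms and encounters.
; Its single function, AddSaveInfos, copies the passed-in deck, player stats, map position, global card ID, encounter type, biom progression data, relics and madness effects into matching variables.
; The function only assigns values, with no disk writing or loading in its graph.
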(fn `AddSaveInfos`
  (params (RunDeck :type "Array of /Game/OldOnes/Core/Cards/SCardData Structure") (PlayerStats :type "/Game/OldOnes/Core/Player/SPlayerState Structure") (InexInWorldMap :type Integer) (GlobalCardID :type Integer) (CurrentEncounterType :type "/Game/OldOnes/Core/GameSettings/EEncounterType Enum" :default "NewEnumerator0") (CurrentBiom :type "/Game/OldOnes/Core/GameSettings/EBiomType Enum" :default "NewEnumerator3") (BiomsDataTables :type "Map of /Game/OldOnes/Core/GameSettings/EBiomType Enum to /Game/OldOnes/Core/RoomSetup/SEnemyRoomsDT Structure") (BiomLevel :type "Map of /Game/OldOnes/Core/GameSettings/EBiomType Enum to Name") (BiomIndexChange :type "Map of Integer to /Game/OldOnes/Core/GameSettings/EBiomType Enum") (Relics :type "Array of Boolean") (MadnessEffects :type "Array of Boolean"))
  (`|ExecutionSequence`
    (:`then_0`
      (set `self.RunDeck` RunDeck))
    (:`then_1`
      (set `self.PlayerStats` PlayerStats))
    (:`then_2`
      (set `self.IndexInWorldMap` InexInWorldMap))
    (:`then_3`
      (set `self.GlobalCardID` GlobalCardID))
    (:`then_4`
      (set `self.CurrentEncounterType` CurrentEncounterType))
    (:`then_5`
      (set `self.CurrentBiom` CurrentBiom))
    (:`then_6`
      (set `self.BiomsDataTables` BiomsDataTables))
    (:`then_7`
      (set `self.BiomLevel` BiomLevel))
    (:`then_8`
      (set `self.BiomsIndexChange` BiomIndexChange))
    (:`then_9`
      (set `self.Relics` Relics))
    (:`then_10`
      (set `self.MadnessEffects` MadnessEffects))))