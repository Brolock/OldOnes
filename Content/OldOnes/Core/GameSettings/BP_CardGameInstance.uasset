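; Game instance for a card game that holds the player's current run deck and supplies the starting deck.
; The run deck is updated by packing the card player pawn's deck into a struct, and is returned on request.
; The starting deck comes from a data table row referenced in the game settings data asset, converted into a deck on lookup.
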(fn `GetRunDeck`
  (returns (RunDeck :type "Array of /Game/OldOnes/Core/Cards/SCardData Structure"))
  (return (`self.RunDeck`)))

(fn `GetStartingDeck`
  (returns (LoadedDeck :type "Array of /Game/OldOnes/Core/Cards/SCardData Structure"))
  (bind (_datatable _rowname) (break `DataTableRowHandle` (`/Game/OldOnes/Core/GameSettings/GameSettings_DataAsset.PlayerStartingDeck` (`self.GameSettingsDataAsset`))))
  (bind _returnvalue (`|GetDataTableRow` _datatable _rowname)
    (:`then`
      (bind _loadeddeck (`/Game/OldOnes/Core/Tools/BPFL_Save.LoadDeckFromDataTableStruct` _returnvalue))
      (return _loadeddeck))))

(fn `UpdateRunDeck`
  (bind _deckstruct (`/Game/OldOnes/Core/Player/BP_PlayerPawn.PackDeckToStruct` (`/Game/OldOnes/Core/Tools/BPFL_GeneralFunctions.GetCardPlayerPawn`)))
  (set `self.RunDeck` _deckstruct))