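; Game mode for the card game that runs turn-based encounters between the player and enemies.
; On BeginPlay it temporarily finds placed enemies, investigables and the player model, builds a player-first turn order and starts the game.
; It binds character end-turn and death-threshold events to advance turns, count rounds and remove the dead.
; The game ends when the player falls or no enemies remain, with only placeholder win/loss messages.
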(event `self.ReceiveBeginPlay`
  (bind _turnorder (`self.TurnOrder`))
  (`KismetSystemLibrary.Delay` 1.0) ; To change once I have figured out enemy spawns
  (set `self.BetweenTurnsDelay` (`/Game/OldOnes/Core/GameSettings/GameSettings_DataAsset.BetweenTurnsDelay` (`/Game/OldOnes/Core/Tools/BPFL_GeneralFunctions.GetGameSettingsDataAsset`)))
  (set `self.Player` (`/Game/OldOnes/Core/Tools/BPFL_GeneralFunctions.GetCardPlayerPawn`))
  (bind _outactors (`GameplayStatics.GetAllActorsOfClass` "/Game/OldOnes/Core/Player/BP_Player3DModel.BP_Player3DModel_C")) ; Temporary way of finding the player's 3D model instead of placing it in the world
  (set `self.Player3DModel` (`|GetArrayItem` _outactors))
  (bind _outactors_2 (`GameplayStatics.GetAllActorsOfClass` "/Game/OldOnes/Core/Enemy/BP_Enemy.BP_Enemy_C")) ; Temporary way of filling the enemies instead of spawning them
  (set `self.Enemies` _outactors_2)
  (bind _outactors_3 (`GameplayStatics.GetAllActorsOfClass` "/Game/OldOnes/Core/Investigable/BP_Investigable.BP_Investigable_C")) ; Temporary way of filling the enemies instead of spawning them
  (set `self.Investigables` _outactors_3)
  (`KismetArrayLibrary.Array_Add` _turnorder (`self.Player`))
  (`KismetArrayLibrary.Array_Append` _turnorder (`self.Enemies`))
  (`self.BindToCharactersEvents` (`self.TurnOrder`))
  (`self.StartGame`))

(event `self.ReceiveTick`
  (params (DeltaSeconds :type "Float (single-precision)")))

(event `CharacterEndTurnEventDelay`
  (params (FiringPawn :type "/Game/OldOnes/Core/Player/BP_BasePawn Object Reference"))
  (`KismetSystemLibrary.Delay` (`self.BetweenTurnsDelay`))
  (`self.CharacterEndTurn` FiringPawn))

(fn `BindToCharactersEvents`
  (params (CharactersToBindTo :type "Array of /Game/OldOnes/Core/Player/BP_BasePawn Object Reference"))
  (for _array_element CharactersToBindTo
    (add `/Game/OldOnes/Core/Player/BP_BasePawn.CharacterDeathThresholdReachedEvent` _array_element (`|CreateDelegate` :!event `CharacterDeathThresholdReceived`))
    (add `/Game/OldOnes/Core/Player/BP_BasePawn.CharacterEndTurnEvent` _array_element (`|CreateDelegate` :!event `CharacterEndTurnEventDelay`))))

(fn `CharacterDeathThresholdReceived`
  (params (FiringPawn :type "/Game/OldOnes/Core/Player/BP_BasePawn Object Reference"))
  (locals (NextCharacterToPlay :type "/Game/OldOnes/Core/Player/BP_BasePawn Object Reference"))
  (bind _firingpawn (`local.FiringPawn`))
  (bind _returnvalue (`KismetArrayLibrary.Array_Find` (`self.TurnOrder`) (`local.NextCharacterToPlay`)))
  (if (== FiringPawn (`self.GetActiveCharacter`))
    (set `local.NextCharacterToPlay` (`self.GetNextCharacterToPlay`))
    (`self.RemoveCharacterFromPlay` _firingpawn)
    (if (not (`self.GameEnded`))
      (bind _output_get (set `self.TurnIndex` _returnvalue))
      (if (== _output_get 0)
        (`/Engine/EditorBlueprintResources/StandardMacros.IncrementInt` (`self.TurnNumber`)
          (:`  `
            _)))
      (`/Game/OldOnes/Core/Player/BP_BasePawn.StartTurn` (`|GetArrayItem` (`self.TurnOrder`) _returnvalue)))
    (else
      (`self.RemoveCharacterFromPlay` _firingpawn))))

(fn `CharacterEndTurn`
  (params (FiringPawn :type "/Game/OldOnes/Core/Player/BP_BasePawn Object Reference"))
  (bind _output_get (set `self.TurnIndex` (mod (+ (`self.TurnIndex`) 1) (`KismetArrayLibrary.Array_Length` (`self.TurnOrder`)))))
  (if (== _output_get 0)
    (`/Engine/EditorBlueprintResources/StandardMacros.IncrementInt` (`self.TurnNumber`) ; Every character has played
      (:`  `
        _)))
  (`/Game/OldOnes/Core/Player/BP_BasePawn.StartTurn` (`|GetArrayItem` (`self.TurnOrder`) _output_get)))

(fn `EndGame`
  (params (PlayerWon :type Boolean))
  (`KismetSystemLibrary.PrintString` "BP_GameMode::EndGame NEED TO CODE AN END GAME SCREEN")
  (set `self.GameEnded` true)
  (`KismetArrayLibrary.Array_Clear` (`self.TurnOrder`))
  (`/Game/OldOnes/Core/Player/BP_BasePawn.EndGame` (`self.Player`)))

(fn `GetActiveCharacter`
  (returns (Output :type "/Game/OldOnes/Core/Player/BP_BasePawn Object Reference"))
  (return (`|GetArrayItem` (`self.TurnOrder`) (`self.TurnIndex`))))

(fn `GetNextCharacterToPlay`
  (returns (NextCharacter :type "/Game/OldOnes/Core/Player/BP_BasePawn Object Reference") (IndexInArray :type Integer))
  (bind _turnorder (`self.TurnOrder`))
  (bind _returnvalue (mod (+ (`self.TurnIndex`) 1) (`KismetArrayLibrary.Array_Length` _turnorder)))
  (return (`|GetArrayItem` _turnorder _returnvalue) _returnvalue))

(fn `IsPlayerTurn`
  (returns (PlayerActive :type Boolean))
  (return (== (`|GetArrayItem` (`self.TurnOrder`) (`self.TurnIndex`)) (`self.Player`))))

(fn `RemoveCharacterFromPlay`
  (params (CharacterToRemove :type "/Game/OldOnes/Core/Player/BP_BasePawn Object Reference"))
  (`KismetArrayLibrary.Array_RemoveItem` (`self.TurnOrder`) CharacterToRemove)
  (if (== CharacterToRemove (`self.Player`))
    (`/Game/OldOnes/Core/Tools/BPFL_WidgetUtilities.Display Message to User` "You've Lost, But we don't do anything about it yet. So just restart? Idk")
    (`self.EndGame` false)
    (else
      (bind _asbp_enemy (cast `/Game/OldOnes/Core/Enemy/BP_Enemy` (`local.CharacterToRemove`)))
      (`KismetArrayLibrary.Array_RemoveItem` (`self.Enemies`) _asbp_enemy)
      (`/Game/OldOnes/Core/Player/BP_BasePawn.Die` _asbp_enemy)
      (if (== (`KismetArrayLibrary.Array_Length` (`self.Enemies`)) 0)
        (`/Game/OldOnes/Core/Tools/BPFL_WidgetUtilities.Display Message to User` "You've Won! We don't do nothing about it yet. So just restart? Idk")
        (`self.EndGame` true)))))

(fn `StartGame`
  (for _array_element (`self.TurnOrder`)
    (`/Game/OldOnes/Core/Player/BP_BasePawn.StartGame` _array_element))
  (`/Game/OldOnes/Core/Player/BP_BasePawn.StartTurn` (`self.GetActiveCharacter`)))

(fn `UserConstructionScript`)