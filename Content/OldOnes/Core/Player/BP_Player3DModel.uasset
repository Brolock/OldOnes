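; BP_Player3DModel is the player's 3D character model, playing animations for idle, attack, damage and death in a card game.
; InitializeModel supplies the skeletal mesh and animation dictionary that each animation lookup uses.
; Attack cards play an animation, with Tick forcing the pawn's PlayCard after a maximum delay if still waiting; other card types play immediately.
; Tick also restarts idle whenever nothing is playing, a stopgap until a proper animation system exists.
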(event `self.ReceiveBeginPlay`
  (set `self.MaximumAnimationDelay` (`/Game/OldOnes/Core/GameSettings/GameSettings_DataAsset.MaximumAnimationDelay` (`/Game/OldOnes/Core/Tools/BPFL_GeneralFunctions.GetGameSettingsDataAsset`))))

(event `self.ReceiveTick`
  (params (DeltaSeconds :type "Float (single-precision)"))
  (bind (_softanimationsequence _animation_found) (`/Game/OldOnes/Core/Tools/BPFL_GeneralFunctions.GetAnimationFromDict` "NewEnumerator0" (`self.AnimationsDict`)))
  (`self.WaitBeforeAbilityExecution` DeltaSeconds)
  ;[1 0.004897 0] HackyWay of playing the idle animation, to change when we have a proper animation system
  (if (`SkeletalMeshComponent.IsPlaying` (`self.SkeletalMesh`))
    _
    (elif _animation_found
      (`SkeletalMeshComponent.PlayAnimation` (`self.SkeletalMesh`) _softanimationsequence false))))

(fn `CallPlayerToPlayCard`
  (set `self.WaitingForAnimationToExecute` false)
  (`/Game/OldOnes/Core/Player/BP_PlayerPawn.Play Card` (`/Game/OldOnes/Core/Tools/BPFL_GeneralFunctions.GetCardPlayerPawn`)))

(fn `Die`
  (bind (_softanimationsequence _animation_found) (`/Game/OldOnes/Core/Tools/BPFL_GeneralFunctions.GetAnimationFromDict` "NewEnumerator3" (`self.AnimationsDict`)))
  (if _animation_found
    (`SkeletalMeshComponent.PlayAnimation` (`self.SkeletalMesh`) _softanimationsequence false)))

(fn `InitializeModel`
  (params (SkeletalMesh :type "SkeletalMesh Object Reference") (AnimationsDict :type "Map of /Game/OldOnes/Core/3D/Animations/EAnimationsTypes Enum to /Game/OldOnes/Core/3D/Animations/SAnimationsArray Structure"))
  (returns (InitializedModel :type "Self Object Reference"))
  (set `self.AnimationsDict` AnimationsDict)
  (`SkinnedMeshComponent.SetSkinnedAssetAndUpdate` (`self.SkeletalMesh`) SkeletalMesh true)
  (return self))

(fn `PlayCardAnimation`
  (params (CardBeingPlayed :type "/Game/OldOnes/Core/Cards/BP_Card Object Reference"))
  (bind (_softanimationsequence _animation_found) (`/Game/OldOnes/Core/Tools/BPFL_GeneralFunctions.GetAnimationFromDict` "NewEnumerator1" (`self.AnimationsDict`)))
  (set `self.WaitingForAnimationToExecute` true)
  (set `self.WaitingTime` 0.0)
  (switch `/Game/OldOnes/Core/Cards/ECardTypes` (`/Game/OldOnes/Core/Cards/BP_Card.GetCardType` CardBeingPlayed)
    (:`NewEnumerator0`
      (if _animation_found
        (`SkeletalMeshComponent.PlayAnimation` (`self.SkeletalMesh`) _softanimationsequence false)
        (else
          (`self.CallPlayerToPlayCard`))))
    (:`NewEnumerator1`
      (`self.CallPlayerToPlayCard` :!label _label))
    (:`NewEnumerator2`
      (goto _label))
    (:`NewEnumerator3`
      (goto _label))
    (:`NewEnumerator5`
      (goto _label))))

(fn `TakeDamage`
  (bind (_softanimationsequence _animation_found) (`/Game/OldOnes/Core/Tools/BPFL_GeneralFunctions.GetAnimationFromDict` "NewEnumerator2" (`self.AnimationsDict`)))
  (if _animation_found
    (`SkeletalMeshComponent.PlayAnimation` (`self.SkeletalMesh`) _softanimationsequence false)))

(fn `UserConstructionScript`)

(fn `WaitBeforeAbilityExecution`
  (params (DeltaTime :type "Float (double-precision)"))
  (if (`self.WaitingForAnimationToExecute`)
    (bind _output_get (set `self.WaitingTime` (+ DeltaTime (`self.WaitingTime`))))
    (if (>= _output_get (`self.MaximumAnimationDelay`))
      (`self.CallPlayerToPlayCard`))))