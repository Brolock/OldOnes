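; Player controller for the card game that turns left mouse input into clicks on enemies and investigables and releases of dragged cards.
; On press, a cursor trace on two object types fires click events for living enemies or investigables.
; Investigable clicks also open the fight UI popup when no targeting or reward pick is active and investigation is allowed.
; On release during fight encounters, it ends the grab on any dragged card.
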(event `self.ReceiveBeginPlay`)

(event `self.ReceiveTick`
  (params (DeltaSeconds :type "Float (single-precision)")))

(event `Key|LeftMouseButton`
  (params (Key :type "Key Structure"))
  (bind (_hitresult _returnvalue) (`self.GetHitResultUnderCursorForObjects` (`|MakeArray` "ObjectTypeQuery7" "ObjectTypeQuery8" :!type "EObjectTypeQuery Enum")))
  (bind (_bblockinghit _binitialoverlap _time _distance _location _impactpoint _normal _impactnormal _physmat _hitactor) (`GameplayStatics.BreakHitResult` _hitresult))
  (:`Pressed`
    (if _returnvalue
      (bind _asbp_enemy (cast `/Game/OldOnes/Core/Enemy/BP_Enemy` _hitactor)
        (:`then`
          (if (`/Game/OldOnes/Core/Enemy/BP_Enemy.IsAlive` _asbp_enemy)
            (`self.EnemyClickedEvent` _asbp_enemy)))
        (:`CastFailed`
          (bind _asbp_investigable (cast `/Game/OldOnes/Core/Investigable/BP_Investigable` _hitactor)
            (:`then`
              (`self.InvestigableClickedEvent` _asbp_investigable)
              (if (and (not (`/Game/OldOnes/Core/Tools/BPFL_GeneralFunctions.IsPlayerChosingTargets`)) (not (`/Game/OldOnes/Core/Tools/BPFL_GeneralFunctions.IsPlayerPickingReward`)) (`/Game/OldOnes/Core/Investigable/BP_Investigable.Is Investigable` _asbp_investigable))
                (set `self.InvestigableClicked` _asbp_investigable)
                (`MenuAnchor.ToggleOpen` (`/Game/OldOnes/Core/PlayerUI/WBP_FightModeUI.InvestigablePopUp` (`/Game/OldOnes/Core/Tools/BPFL_GeneralFunctions.GetFightModeUI`)) true)))
            (:`CastFailed`
              (`KismetSystemLibrary.PrintString` "BP_CardPlayerController::EventLeftMouse: triggered an unknown actor with collision OldOnesEnemy/Investigable"))))))))

(event `Key|LeftMouseButton`
  (params (Key :type "Key Structure"))
  (bind _draggedcard (`/Game/OldOnes/Core/PlayerUI/WBP_FightModeUI.DraggedCard` (`/Game/OldOnes/Core/Tools/BPFL_GeneralFunctions.GetFightModeUI`)))
  (:`Released`
    (if (`/Game/OldOnes/Core/Tools/BPFL_GeneralFunctions.IsEncounterTypeFight`)
      (`/Engine/EditorBlueprintResources/StandardMacros.IsValid` _draggedcard
        (:`Is Valid`
          (`/Game/OldOnes/Core/PlayerUI/WBP_CardView.StopGrab` _draggedcard false))))))

(fn `UserConstructionScript`)