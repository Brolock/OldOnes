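; Player pawn for the card battler, holding the player's deck and fight stats: HP, block, mana, Investigation and Madness.
; Cards move between draw, discard and exile piles and the HandManager, reshuffling discards when the draw pile empties.
; Turn overrides handle redraw, mana refill and block resets, while stat setters fire change events and card plays go through the 3D model's animation when present.
; State loads from and packs into structs.
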(event `self.ReceiveBeginPlay`
  (`parent.ReceiveBeginPlay`))

(fn `CanDraw`
  (returns (CanDraw :type Boolean) (CantDrawMessage :type String))
  (if (`self.IsHandFull`)
    (return false "Hand is full")
    (elif (and (`/Game/OldOnes/Core/CardPile/BP_CardPile.IsEmpty` (`self.DrawPile`)) (`/Game/OldOnes/Core/CardPile/BP_CardPile.IsEmpty` (`self.DiscardPile`)))
      (return false "Draw and Discard Piles are empty")
      (else
        (return true "")))))

(fn `CardReadyForPlay`
  (params (CardToPlay :type "/Game/OldOnes/Core/Cards/BP_Card Object Reference") (PayMana :type Boolean :default true))
  (if PayMana
    (`self.PayMana` (`/Game/OldOnes/Core/Cards/BP_Card.GetManaValue` CardToPlay)))
  (bind _output_get (set `self.CardBeingPlayed` CardToPlay))
  (`/Engine/EditorBlueprintResources/StandardMacros.IsValid` (`self.3DModel`)
    (:`Is Valid`
      (`/Game/OldOnes/Core/Player/BP_Player3DModel.PlayCardAnimation` (`self.3DModel`) _output_get))
    (:`Is Not Valid`
      (`self.Play Card`))))

(fn `ChangeInvestigation`
  (params (NewInvestigation :type Integer))
  (locals (AmountChanged :type Integer))
  (bind _output_get (set `local.AmountChanged` (- NewInvestigation (`self.Investigation`))))
  (bind _output_get_2 (set `self.Investigation` NewInvestigation))
  (`self.ChangeInvestigationEvent` _output_get _output_get_2))

(fn `ChangeMadness`
  (params (NewMadnessValue :type Integer))
  (locals (AmountChanged :type Integer))
  (bind _output_get (set `local.AmountChanged` (- NewMadnessValue (`self.Madness`))))
  (bind _output_get_2 (set `self.Madness` NewMadnessValue))
  (`self.ChangeMadnessEvent` _output_get _output_get_2))

(fn `ChangeMana`
  (params (NewManaValue :type Integer))
  (locals (AmountChanged :type Integer))
  (bind _output_get (set `local.AmountChanged` (- NewManaValue (`self.CurrentMana`))))
  (bind _output_get_2 (set `self.CurrentMana` NewManaValue))
  (`self.ChangeManaEvent` _output_get _output_get_2))

(fn `ChangeManaPerTurn`
  (params (NewMaxMan :type Integer))
  (locals (AmountChanged :type Integer))
  (bind _output_get (set `local.AmountChanged` (- NewMaxMan (`self.ManaPerTurn`))))
  (bind _output_get_2 (set `self.ManaPerTurn` NewMaxMan))
  (`self.ChangeManaEvent` _output_get _output_get_2))

(fn `Die`
  (`parent.Die`)
  (`/Game/OldOnes/Core/Player/BP_Player3DModel.Die` (`self.3DModel`)))

(fn `DiscardCard`
  (params (Card :type "/Game/OldOnes/Core/Cards/BP_Card Object Reference"))
  (bind (_removedcard _wassuccessful) (`/Game/OldOnes/Core/CardPile/BP_HandManager.RemoveFromHand` (`self.HandManager`) Card))
  (if _wassuccessful
    (`/Game/OldOnes/Core/CardPile/BP_CardPile.AddCardToPile` (`self.DiscardPile`) _removedcard "NewEnumerator0" false)
    (else
      (`KismetSystemLibrary.PrintString` "BP_CardPlayerPawn::Discard: Trying to discard a card that is not in hand?" true true (struct :`G` 0.66 :`B` 1.0 :`A` 1.0) 20.0))))

(fn `DiscardHand`
  (bind _removedcards (`/Game/OldOnes/Core/CardPile/BP_HandManager.RemoveAllCardsFromHand` (`self.HandManager`)))
  (`KismetArrayLibrary.Array_Reverse` _removedcards)
  (`/Game/OldOnes/Core/CardPile/BP_CardPile.AddCardsToPile` (`self.DiscardPile`) _removedcards "NewEnumerator0"))

(fn `DrawCard`
  (returns (CardDrawn :type "/Game/OldOnes/Core/Cards/BP_Card Object Reference"))
  (bind (_candraw _cantdrawmessage) (`self.CanDraw`))
  ;[1 1 1] Shuffle discard to deck if Draw pile is empty
  (if _candraw
    (if (`/Game/OldOnes/Core/CardPile/BP_CardPile.IsEmpty` (`self.DrawPile`))
      (`self.ShuffleDiscardToDeck`))
    (bind (_carddrawn _cardvalid) (`/Game/OldOnes/Core/CardPile/BP_CardPile.DrawCard` (`self.DrawPile`)))
    (if _cardvalid
      (`/Game/OldOnes/Core/CardPile/BP_HandManager.AddCardToHand` (`self.HandManager`) _carddrawn)
      (return _carddrawn)
      (else
        (return null)))
    (else
      (`/Game/OldOnes/Core/Tools/BPFL_WidgetUtilities.Display Message to User (String)` _cantdrawmessage)
      (return null))))

(fn `DrawCards`
  (params (AmountToDraw :type Integer))
  (returns (NumberOfCardsDrawn :type Integer) (CardsDrawn :type "Array of /Game/OldOnes/Core/Cards/BP_Card Object Reference"))
  (locals (CardsDrawnLocal :type "Array of /Game/OldOnes/Core/Cards/BP_Card Object Reference") (NbCardsDrawn :type Integer) (LastCardValid :type Boolean :default true))
  (if (> AmountToDraw 0)
    (while (and (< (`local.NbCardsDrawn`) (`local.AmountToDraw`)) (`local.LastCardValid`))
      (bind _carddrawn (`self.DrawCard`))
      (bind _output_get (set `local.LastCardValid` (`KismetSystemLibrary.IsValid` _carddrawn)))
      (if _output_get
        (`KismetArrayLibrary.Array_Add` (`local.CardsDrawnLocal`) _carddrawn)
        (`/Engine/EditorBlueprintResources/StandardMacros.IncrementInt` (`local.NbCardsDrawn`))))
    (return (`local.NbCardsDrawn`) (`local.CardsDrawnLocal`))))

(fn `EndGame`
  (`parent.EndGame`)
  (set `self.CurrentMana` 0)
  (set `self.Investigation` 0))

(fn `EndTurn`
  (`parent.EndTurn`)
  (set `self.BaseActions` true)
  (`self.DiscardHand`)
  (`self.DrawCards` (`self.CardsPerTurn`))
  (`self.ChangeMana` 0) ; ResetMana function could be put later
  (`self.ChangeMana` (+ (`self.CurrentMana`) (`self.ManaPerTurn`)))
  (bind _enemies (`/Game/OldOnes/Core/Tools/BPFL_Targeting.GetAllEnemies`))
  ;[0.09705 0.8298 1] Reset enemy shields at the end of the player turn.
  (for _array_element _enemies
    (bind _output_get (set `/Game/OldOnes/Core/Player/BP_BasePawn.Block` 0 _array_element))
    (`self.BlockTakenEvent` _array_element 0 _output_get))
  (set `self.BaseActions` false)
  (`self.CharacterEndTurnEvent` self)
  (return))

(fn `GainInvestigatePoints`
  (params (Amount :type Integer))
  (returns (AmountGained :type Integer))
  (`self.ChangeInvestigation` (+ Amount (`self.Investigation`)))
  (return Amount))

(fn `GetPileFromLocation`
  (params (PileLocation :type "/Game/OldOnes/Core/Cards/ECardLocation Enum" :default "NewEnumerator0"))
  (returns (CardPile :type "/Game/OldOnes/Core/CardPile/BP_CardPile Object Reference"))
  (switch `/Game/OldOnes/Core/Cards/ECardLocation` PileLocation
    (:`NewEnumerator0`
      (return (`self.DrawPile`)))
    (:`NewEnumerator1`
      (return (`self.DiscardPile`)))
    (:`NewEnumerator2`
      _)
    (:`NewEnumerator3`
      (return (`self.ExilePile`)))
    (:`NewEnumerator4`
      _))
  (`KismetSystemLibrary.PrintString` "BP_PlayerPawn::GetPileFromLocation: Hand or play are not a pile locations" true true (struct :`A` 1.0) 20.0))

(fn `Initialize Player From State Struct`
  (params (PlayerStateStruct :type "/Game/OldOnes/Core/Player/SPlayerState Structure"))
  (bind (_startinghp _maxhp _startingblock) (break `/Game/OldOnes/Core/Player/SPlayerState` (`local.PlayerStateStruct`)))
  (bind (_startinghp_2 _maxhp_2 _startingblock_2 _startingmana _manaperturn _cardsperturn _maxhandsize) (break `/Game/OldOnes/Core/Player/SPlayerState` (`local.PlayerStateStruct`)))
  (bind (_startinghp_3 _maxhp_3 _startingblock_3 _startingmana_2 _manaperturn_2 _cardsperturn_2 _maxhandsize_2 _startinginvestigation _startingmadness _maxmadness) (break `/Game/OldOnes/Core/Player/SPlayerState` (`local.PlayerStateStruct`)))
  (`|ExecutionSequence`
    (:`then_0`
      ;[0.4437 1 0.3343] Pawn stats
      (set `self.CurrentHP` _startinghp)
      (set `self.MaxHP` _maxhp)
      (set `self.Block` _startingblock))
    (:`then_1`
      ;[0.4656 0.3146 1] Player Stats
      (set `self.CurrentMana` _startingmana)
      (set `self.ManaPerTurn` _manaperturn)
      (set `self.CardsPerTurn` _cardsperturn)
      (bind _output_get (set `self.MaxHandSize` _maxhandsize))
      (set `/Game/OldOnes/Core/CardPile/BP_HandManager.MaxHandSize` _output_get (`self.HandManager`)))
    (:`then_2`
      ;[0.5938 0.07606 0.02875] OldOnes Specific Stats
      (set `self.Investigation` _startinginvestigation)
      (set `self.Madness` _startingmadness)
      (set `self.MaxMadness` _maxmadness))))

(fn `Initialize3DModel`
  (params (`3DModel` :type "/Game/OldOnes/Core/Player/BP_Player3DModel Object Reference"))
  (set `self.3DModel` `3DModel`))

(fn `InitializeCardViews`
  (`/Game/OldOnes/Core/CardPile/BP_CardPile.Initialize Cards Views` (`self.DrawPile`) (`/Game/OldOnes/Core/PlayerUI/WBP_FightModeUI.DrawPile` (`self.FightModeUI`)))
  (`/Game/OldOnes/Core/CardPile/BP_CardPile.Initialize Cards Views` (`self.DiscardPile`) (`/Game/OldOnes/Core/PlayerUI/WBP_FightModeUI.DiscardPile` (`self.FightModeUI`)))
  (`/Game/OldOnes/Core/CardPile/BP_CardPile.Initialize Cards Views` (`self.ExilePile`) (`/Game/OldOnes/Core/PlayerUI/WBP_FightModeUI.ExilePile` (`self.FightModeUI`))))

(fn `InitializeFightDeck`
  (params (DeckStruct :type "/Game/OldOnes/Core/CardPile/BP_CardPile Object Reference"))
  (bind _cardsstruct (`/Game/OldOnes/Core/CardPile/BP_CardPile.PackCardsToStruct` DeckStruct))
  (for _array_element _cardsstruct
    (bind _initializedcard (`/Game/OldOnes/Core/Tools/BPFL_Cards.CreateCardFromStruct` _array_element self))
    (`/Game/OldOnes/Core/CardPile/BP_CardPile.AddCardToPile` (`self.DrawPile`) _initializedcard "NewEnumerator0" true))
  (set `self.FightModeUI` (`/Game/OldOnes/Core/GameUI/WBP_GameUI.FightModeUI` (`/Game/OldOnes/Core/Tools/BPFL_GeneralFunctions.GetGameUI`)))
  (`/Game/OldOnes/Core/PlayerUI/WBP_FightModeUI.InitFightUI` (`self.FightModeUI`) self)
  (`self.InitializeCardViews`))

(fn `Investigate`
  (params (Investigable :type "/Game/OldOnes/Core/Investigable/BP_Investigable Object Reference"))
  (bind _pointsused (`/Game/OldOnes/Core/Investigable/BP_Investigable.Investigate` Investigable (`KismetMathLibrary.Min` (`self.Investigation`) 5)))
  (`self.LoseInvestigatePoints` _pointsused))

(fn `IsHandFull`
  (returns (ReturnValue :type Boolean))
  (return (`/Game/OldOnes/Core/CardPile/BP_HandManager.IsHandFull` (`self.HandManager`))))

(fn `LoseInvestigatePoints`
  (params (Amount :type Integer))
  (returns (AmountLost :type Integer))
  (locals (AmountLostLocal :type Integer))
  (bind _output_get (set `local.AmountLostLocal` (`KismetMathLibrary.Min` Amount (`self.Investigation`))))
  (`self.ChangeInvestigation` (- (`self.Investigation`) _output_get))
  (return (`local.AmountLostLocal`)))

(fn `PackDeckToStruct`
  (returns (DeckStruct :type "Array of /Game/OldOnes/Core/Cards/SCardData Structure"))
  (locals (DeckStructLocal :type "Array of /Game/OldOnes/Core/Cards/SCardData Structure"))
  (bind _cardsstruct (`/Game/OldOnes/Core/CardPile/BP_CardPile.PackCardsToStruct` (`self.DrawPile`))) ; Draw
  (`KismetArrayLibrary.Array_Append` (`local.DeckStructLocal`) _cardsstruct)
  (bind _cardsstruct_2 (`/Game/OldOnes/Core/CardPile/BP_CardPile.PackCardsToStruct` (`self.DiscardPile`))) ; Discard
  (`KismetArrayLibrary.Array_Append` (`local.DeckStructLocal`) _cardsstruct_2)
  (bind _cardsstruct_3 (`/Game/OldOnes/Core/CardPile/BP_CardPile.PackCardsToStruct` (`self.ExilePile`))) ; Exile
  (`KismetArrayLibrary.Array_Append` (`local.DeckStructLocal`) _cardsstruct_3)
  (bind _cardsstruct_4 (`/Game/OldOnes/Core/CardPile/BP_HandManager.PackCardsToStruct` (`self.HandManager`))) ; Hand
  (`KismetArrayLibrary.Array_Append` (`local.DeckStructLocal`) _cardsstruct_4)
  (return (`local.DeckStructLocal`)))

(fn `PackSelfToStruct`
  (returns (PlayerStateStruct :type "/Game/OldOnes/Core/Player/SPlayerState Structure"))
  (bind (_startinghp _maxhp _startingblock _startingmana _manaperturn _cardsperturn _maxhandsize _startinginvestigation _startingmadness _maxmadness) (break `/Game/OldOnes/Core/Player/SPlayerState` (`/Game/OldOnes/Core/Tools/BPFL_GeneralFunctions.GetRunPlayerStats`)))
  (return (make `/Game/OldOnes/Core/Player/SPlayerState` (`self.CurrentHP`) _maxhp _startingblock _startingmana _manaperturn _cardsperturn _maxhandsize _startinginvestigation (`self.Madness`) _maxmadness)))

(fn `PayMana`
  (params (Amount :type Integer))
  (`self.ChangeMana` (- (`self.CurrentMana`) Amount)))

(fn `PickCard`
  (params (CardToPick :type "/Game/OldOnes/Core/Cards/BP_Card Object Reference"))
  (returns (CardPicked :type Boolean))
  (locals (ShouldShuffle :type Boolean))
  (bind _cardlocation (`/Game/OldOnes/Core/Cards/BP_Card.CardLocation` CardToPick))
  (if (not (`self.IsHandFull`))
    (set `local.ShouldShuffle` (`|EnumEquality` _cardlocation "NewEnumerator0"))
    (bind (_removedcard _cardremoved) (`/Game/OldOnes/Core/CardPile/BP_CardPile.RemoveCardFromPile` (`self.GetPileFromLocation` _cardlocation) (`local.CardToPick`)))
    (if _cardremoved
      (`/Game/OldOnes/Core/CardPile/BP_HandManager.AddCardToHand` (`self.HandManager`) _removedcard)
      (if (`local.ShouldShuffle`)
        (`/Game/OldOnes/Core/CardPile/BP_CardPile.Shuffle` (`self.DrawPile`)))
      (return true)
      (else
        _)))
  (return false))

(fn `Play Card`
  (bind _cardbeingplayed (`self.CardBeingPlayed`))
  (`/Game/OldOnes/Core/Cards/BP_Card.PlayCard` _cardbeingplayed)
  (`self.DiscardCard` _cardbeingplayed)
  (set `self.CardBeingPlayed` null))

(fn `ResetPlayer_GameReset`
  (bind _3dmodel (`self.3DModel`))
  (set `self.BaseActions` false)
  ;[1 0 0] ResetPlayer UI Could be optimized for performance (keeping cards widget for example)
  (`/Game/OldOnes/Core/PlayerUI/WBP_FightModeUI.Reset UI Game Reset` (`self.FightModeUI`))
  ;[1 1 1] Destroy Player's 3D model
  (`self.SetActorHiddenInGame` _3dmodel false)
  (`self.K2_DestroyActor` _3dmodel)
  (set `self.3DModel` null)
  ;[1 0 0] Clear all existing cards Could be optimized
  (`|ExecutionSequence`
    (:`then_0`
      (`/Game/OldOnes/Core/CardPile/BP_HandManager.ClearHand_GameReset` (`self.HandManager`)))
    (:`then_1`
      (`/Game/OldOnes/Core/CardPile/BP_CardPile.ClearPile_GameReset` (`self.DrawPile`)))
    (:`then_2`
      (`/Game/OldOnes/Core/CardPile/BP_CardPile.ClearPile_GameReset` (`self.DiscardPile`)))
    (:`then_3`
      (`/Game/OldOnes/Core/CardPile/BP_CardPile.ClearPile_GameReset` (`self.ExilePile`)))))

(fn `ShuffleDiscardToDeck`
  (`/Game/OldOnes/Core/CardPile/BP_CardPile.ChangeCardsPile` (`self.DiscardPile`) (`self.DrawPile`))
  (`/Game/OldOnes/Core/CardPile/BP_CardPile.Shuffle` (`self.DrawPile`)))

(fn `StartGame`
  (`parent.StartGame`)
  (set `/Game/OldOnes/Core/CardPile/BP_HandManager.MaxHandSize` (`self.MaxHandSize`) (`self.HandManager`))
  (set `self.BaseActions` true)
  (`self.DrawCards` (`self.CardsPerTurn`))
  (`self.ChangeMana` (+ (`self.CurrentMana`) (`self.ManaPerTurn`)))
  (set `self.BaseActions` false))

(fn `StartTurn`
  (`parent.StartTurn`)
  (bind _output_get (set `self.Block` 0))
  (`self.BlockTakenEvent` 0 _output_get))

(fn `TakeDamage`
  (params (AmountToTake :type Integer))
  (returns (DamageTaken :type Integer) (BlockTaken :type Integer))
  (bind _3dmodel (`self.3DModel`))
  (`/Engine/EditorBlueprintResources/StandardMacros.IsValid` _3dmodel
    (:`Is Valid`
      (`/Game/OldOnes/Core/Player/BP_Player3DModel.TakeDamage` _3dmodel))
    (:`Is Not Valid`
      _))
  (bind (_damagetaken _blocktaken) (`parent.TakeDamage` AmountToTake))
  (return _damagetaken _blocktaken))

(fn `UserConstructionScript`
  (`parent.UserConstructionScript`))