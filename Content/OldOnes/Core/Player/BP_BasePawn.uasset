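; BP_BasePawn is the base pawn for turn-based combat, holding HP and Block along with the damage, heal and block logic.
; TakeDamage spends Block first and passes the remainder to TakeDirectDamage, which signals the death threshold at zero HP or below.
; Each stat change fires an event dispatcher with the delta and new value.
; StartTurn clears Block, while the game start/end, EndTurn and Die functions are empty stubs.
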(event `self.ReceiveBeginPlay`)

(event `self.ReceiveTick`
  (params (DeltaSeconds :type "Float (single-precision)")))

(fn `Die`)

(fn `EndGame`)

(fn `EndTurn`)

(fn `GainBlock`
  (params (BlockToGain :type Integer))
  (returns (GainedBlock :type Integer))
  (bind _blocktogain (`local.BlockToGain`))
  (bind _output_get (set `self.Block` (+ BlockToGain (`self.Block`))))
  (`self.BlockGainedEvent` _blocktogain _output_get)
  (return _blocktogain))

(fn `Heal`
  (params (AmounToHeal :type Integer))
  (returns (LifeHealed :type Integer))
  (locals (PreHealHP :type Integer))
  (bind _currenthp (`self.CurrentHP`))
  (set `local.PreHealHP` _currenthp)
  (bind _output_get (set `self.CurrentHP` (`KismetMathLibrary.Min` (+ AmounToHeal _currenthp) (`self.MaxHP`))))
  (bind _returnvalue (- _output_get (`local.PreHealHP`)))
  (`self.HealedEvent` _returnvalue _output_get)
  (return _returnvalue))

(fn `StartGame`)

(fn `StartTurn`
  (bind _output_get (set `self.Block` 0))
  (`self.BlockTakenEvent` 0 _output_get))

(fn `TakeDamage`
  (params (AmountToTake :type Integer))
  (returns (DamageTaken :type Integer) (BlockTaken :type Integer))
  (locals (DamageToHp :type Integer) (BlockLost :type Integer))
  (set `local.DamageToHP` (`KismetMathLibrary.Max` (- AmountToTake (`self.Block`))))
  (set `local.BlockLost` (`KismetMathLibrary.Min` (`self.Block`) (`local.AmountToTake`)))
  (set `self.Block` (- (`self.Block`) (`local.BlockLost`)))
  (`self.BlockTakenEvent` (`local.BlockLost`) (`self.Block`))
  (bind _damagetaken (`self.TakeDirectDamage` (`local.DamageToHP`)))
  (return _damagetaken (`local.BlockLost`)))

(fn `TakeDirectDamage`
  (params (AmountOfDamage :type Integer))
  (returns (DamageTaken :type Integer))
  (bind _output_get (set `self.CurrentHP` (- (`self.CurrentHP`) AmountOfDamage)))
  (`self.DamageTakenEvent` AmountOfDamage _output_get)
  (if (not (> (`self.CurrentHP`) 0))
    (`self.CharacterDeathThresholdReachedEvent` self))
  (return (`local.AmountOfDamage`)))

(fn `UserConstructionScript`)